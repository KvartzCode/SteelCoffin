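; Enemy that chases the player character and dies as soon as it overlaps them.
; While it can move and is not dead, Tick re-issues AI MoveTo toward the player; the first successful arrival switches movement off.
; Death disables capsule collision, hides the mesh, plays a death effect, notifies the game mode, and destroys the actor when the effect finishes.
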(event `self.ReceiveBeginPlay`
  ;[1 1 1] Init
  (set `self.PlayerTarget` (`GameplayStatics.GetPlayerCharacter` 0)))

(event `self.ReceiveTick`
  (params (DeltaSeconds :type "Float (single-precision)"))
  ;[1 1 1] Update
  (if (`self.AndNotDead` (`self.CanMove`))
    (`self.FollowPlayer`)))

(event `FollowPlayer`
  ;[1 1 1] Movement
  (`|AIMoveTo` self (0.0 0.0 0.0) (`self.PlayerTarget`) 0.0
    (:`OnSuccess`
      (`/Engine/EditorBlueprintResources/StandardMacros.DoOnce` false
        (:`Completed`
          (set `self.CanMove` false))))))

(event `self.ReceiveActorBeginOverlap`
  (params (OtherActor :type "Actor Object Reference"))
  ;[1 1 1] Enemy touched player
  (if (`self.AndNotDead` (== OtherActor (`GameplayStatics.GetPlayerCharacter` 0)))
    (`/Game/Blueprints/Interfaces/BPI_EnemyInterface.KillEnemy`)))

(event `/Game/Blueprints/Interfaces/BPI_EnemyInterface.KillEnemy`
  (bind _fx_enemydeath (`self.FX_EnemyDeath`))
  (bind _mesh (`self.Mesh`))
  ;[1 1 1] Death Events
  (`PrimitiveComponent.SetCollisionEnabled` (`self.CapsuleComponent`) "NoCollision")
  (set `self.IsDead` true)
  (`SceneComponent.SetVisibility` _mesh false false)
  (`ActorComponent.Deactivate` _mesh)
  (`ActorComponent.Deactivate` (`self.Mesh`))
  (`ActorComponent.Activate` _fx_enemydeath false)
  (add `NiagaraComponent.OnSystemFinished` _fx_enemydeath (delegate `OnSystemFinished`))
  (message `/Game/Blueprints/Interfaces/BPI_GameModeInterface.EnemyKilled` (`GameplayStatics.GetGameMode`) self))

(event `OnSystemFinished`
  (params (PSystem :type "NiagaraComponent Object Reference"))
  ;[1 1 1] Death Events
  (`self.K2_DestroyActor`))

(fn `UserConstructionScript`)