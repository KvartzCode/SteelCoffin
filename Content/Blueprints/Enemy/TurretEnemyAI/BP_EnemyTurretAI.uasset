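; Enemy turret AI pawn that runs a behavior tree on possession, hands its health to the Enemy_Controller and routes incoming damage to that controller.
; Tick writes both gun socket locations and an aiming-mesh key to the blackboard.
; When perception senses the player mech, it flags Sighted, interpolates the middle turret mesh toward the player on that update only, and plays a one-time spotted sound.
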(event `self.ReceivePossessed`
  (params (NewController :type "Controller Object Reference"))
  (bind _returnvalue (`AIBlueprintHelperLibrary.GetAIController` self))
  (`AIController.RunBehaviorTree` _returnvalue "/Game/Blueprints/Enemy/TurretEnemyAI/BT_EnemyTurretAI.BT_EnemyTurretAI")
  (bind _asenemy_controller (cast `/Game/Blueprints/Enemy/BipedalEnemyAI/Enemy_Controller` _returnvalue))
  (set `/Game/Blueprints/Enemy/BipedalEnemyAI/Enemy_Controller.EnemyHealth` (`self.TurretHealth`) _asenemy_controller))

(event `self.ReceiveTick`
  (params (DeltaSeconds :type "Float (single-precision)"))
  (bind _medium_military_turret_top_tubes_l (`self.Medium_Military_turret_TOP_Tubes_L`))
  (set `self.Delta Seconds` DeltaSeconds)
  (`BlackboardComponent.SetValueAsVector` (`AIBlueprintHelperLibrary.GetBlackboard` null) "GunSocketLocation" (`SceneComponent.GetSocketLocation` _medium_military_turret_top_tubes_l "Gun1Socket"))
  (`BlackboardComponent.SetValueAsVector` (`AIBlueprintHelperLibrary.GetBlackboard` null) "AlternateGunSocketLocation" (`SceneComponent.GetSocketLocation` _medium_military_turret_top_tubes_l "Gun2Socket"))
  (`BlackboardComponent.SetValueAsObject` (`AIBlueprintHelperLibrary.GetBlackboard` null) "EnemyAimingMesh" null))

(event `CustomEvent`
  (params (DamageAmount :type "Float (double-precision)"))
  ;[1 1 1] Sends an event to the enemy controller to take damage
  (bind _asenemy_controller (cast `/Game/Blueprints/Enemy/BipedalEnemyAI/Enemy_Controller` (`self.GetController`)))
  (`/Game/Blueprints/Enemy/BipedalEnemyAI/Enemy_Controller.TakeDamage` _asenemy_controller DamageAmount (0.0 0.0 0.0)))

(event `self.AIPerception.OnTargetPerceptionUpdated`
  (params (Actor :type "Actor Object Reference") (Stimulus :type "AIStimulus Structure"))
  (bind _medium_military_turret_middle_vertical_rot_l (`self.Medium_Military_turret_MIDDLE_vertical_rot_L`))
  (bind _asbp_player_mech (cast `/Game/Blueprints/Player/BP_PlayerMech` Actor))
  (if (`.bSuccessfullySensed` (break `AIStimulus` Stimulus))
    (`BlackboardComponent.SetValueAsBool` (`AIBlueprintHelperLibrary.GetBlackboard` null) "Sighted" true)
    (bind (_returnvalue_roll _returnvalue_pitch _returnvalue_yaw) (`KismetMathLibrary.BreakRotator` (`KismetMathLibrary.FindLookAtRotation` (`SceneComponent.K2_GetComponentLocation` (`self.Medium_Military_turret_MIDDLE_vertical_rot_L`)) (`SceneComponent.K2_GetComponentLocation` (`Actor.RootComponent` _asbp_player_mech)))))
    (`SceneComponent.K2_SetWorldRotation` _medium_military_turret_middle_vertical_rot_l (`KismetMathLibrary.RInterpTo` (`SceneComponent.K2_GetComponentRotation` _medium_military_turret_middle_vertical_rot_l) (`KismetMathLibrary.MakeRotator` _returnvalue_roll _returnvalue_pitch _returnvalue_yaw) (`self.Delta Seconds`) (`self.RotationSpeed`)) false false)
    (`/Engine/EditorBlueprintResources/StandardMacros.DoOnce` false
      (:`Completed`
        (`KismetSystemLibrary.PrintString` "Spotted")
        (`GameplayStatics.PlaySoundAtLocation` "/Game/Sounds/Mech/EnemyMech/SFX_EnemyMechTargetAquired.SFX_EnemyMechTargetAquired" (`self.K2_GetActorLocation`) (struct) 1.0 1.0 0.0 null null null null)))))

(event `/Game/Blueprints/Interfaces/BPI_EnemyInterface.DamageEnemy`
  (params (DamageAmount :type "Float (double-precision)") (HitLocation :type "Vector Structure"))
  ;[1 1 1] Sends an event to the enemy controller to take damage
  (bind _asenemy_controller (cast `/Game/Blueprints/Enemy/BipedalEnemyAI/Enemy_Controller` (`self.GetController`)))
  (`/Game/Blueprints/Enemy/BipedalEnemyAI/Enemy_Controller.TakeDamage` _asenemy_controller DamageAmount HitLocation))

(fn `UserConstructionScript`)