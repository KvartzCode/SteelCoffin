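; BP_Enemy_Character is the character Blueprint for a bipedal enemy driven by a behavior tree.
; On possession it runs BT_BipedalEnemy on its AI controller and prints a debug string.
; DamageEnemy forwards damage amount and hit location to Enemy_Controller, while UpdateWalkSpeed sets the movement component's max walk speed.
; Tick is empty, as the nodes writing player distance and target to the blackboard are disconnected.
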(event `self.ReceivePossessed`
  (params (NewController :type "Controller Object Reference"))
  (`AIController.RunBehaviorTree` (`AIBlueprintHelperLibrary.GetAIController` self) "/Game/Blueprints/Enemy/BehaviorTree/BT_BipedalEnemy.BT_BipedalEnemy")
  (`KismetSystemLibrary.PrintString` "Heyo"))

(event `self.ReceiveTick`
  (params (DeltaSeconds :type "Float (single-precision)"))
  ;[1 1 1] Sets and constantly updates the CurrentTargetDistance variable in the blackboard to the distance between the enemy and the player
)

(event `/Game/Blueprints/Interfaces/BPI_EnemyInterface.DamageEnemy`
  (params (DamageAmount :type "Float (double-precision)") (HitLocation :type "Vector Structure"))
  ;[1 1 1] Sends an event to the enemy controller to take damage
  (bind _asenemy_controller (cast `/Game/Blueprints/Enemy/BipedalEnemyAI/Enemy_Controller` (`self.GetController`)))
  (`/Game/Blueprints/Enemy/BipedalEnemyAI/Enemy_Controller.TakeDamage` _asenemy_controller DamageAmount HitLocation))

(fn `UpdateWalkSpeed`
  (params (NewWalkSpeed :type "Float (double-precision)"))
  (set `CharacterMovementComponent.MaxWalkSpeed` NewWalkSpeed (`self.CharacterMovement`)))

(fn `UserConstructionScript`)