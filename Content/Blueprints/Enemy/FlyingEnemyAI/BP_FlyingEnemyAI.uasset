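; Flying drone enemy that runs the BT_FlyingAI behavior tree when possessed and aims its guns at the player.
; On possession it collects six gun pipes and sets the head's relative height from chained random rolls, re-rolled at each branch so odds are uneven.
; Tick smoothly turns DroneGunLeg2 toward the player's mesh; an author note flags the right-vector axis as needing a fix.
; DamageEnemy forwards damage and hit location to Enemy_Controller.
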(event `self.ReceivePossessed`
  (params (NewController :type "Controller Object Reference"))
  (bind _returnvalue (`KismetMathLibrary.RandomIntegerInRange` 1 4))
  (`AIController.RunBehaviorTree` (`AIBlueprintHelperLibrary.GetAIController` self) "/Game/Blueprints/Enemy/FlyingEnemyAI/BT_FlyingAI.BT_FlyingAI")
  (`KismetSystemLibrary.PrintString` "Flying Drone Spawn")
  (set `self.DroneGuns` (`|MakeArray` (`self.DroneGun_pipe1`) (`self.DroneGun_pipe2`) (`self.DroneGun_pipe3`) (`self.DroneGun_pipe4`) (`self.DroneGun_pipe5`) (`self.DroneGun_pipe6`)))
  (if (== _returnvalue 1.0)
    (set `self.ElevationHeight` 300.0)
    (elif (== _returnvalue 2.0)
      (set `self.ElevationHeight` 325.0)
      (elif (== _returnvalue 3.0)
        (set `self.ElevationHeight` 250.0)
        (elif (== _returnvalue 4.0)
          (set `self.ElevationHeight` 225.0)
          (else
            (set `self.ElevationHeight` 275.0))))))
  (`SceneComponent.K2_SetRelativeLocation` (`self.DroneHead_head`) (`KismetMathLibrary.MakeVector` 0.0 0.0 (`self.ElevationHeight`)) false false))

(event `self.ReceiveTick`
  (params (DeltaSeconds :type "Float (single-precision)"))
  (bind _dronegun_leg2 (`self.DroneGun_leg2`))
  (bind (_returnvalue_roll _returnvalue_pitch _returnvalue_yaw) (`KismetMathLibrary.BreakRotator` (`KismetMathLibrary.FindLookAtRotation` (`SceneComponent.K2_GetComponentLocation` (`self.DroneGun_leg2`)) (`SceneComponent.K2_GetComponentLocation` (`Character.Mesh` (`GameplayStatics.GetPlayerCharacter` 0))))))
  (`SceneComponent.K2_SetWorldRotation` _dronegun_leg2 (`KismetMathLibrary.RInterpTo` (`SceneComponent.K2_GetComponentRotation` _dronegun_leg2) (`KismetMathLibrary.MakeRotator` _returnvalue_roll _returnvalue_pitch _returnvalue_yaw) DeltaSeconds 7.5) false false))

(event `/Game/Blueprints/Interfaces/BPI_EnemyInterface.DamageEnemy`
  (params (DamageAmount :type "Float (double-precision)") (HitLocation :type "Vector Structure"))
  ;[1 1 1] Sends an event to the enemy controller to take damage
  (bind _asenemy_controller (cast `/Game/Blueprints/Enemy/BipedalEnemyAI/Enemy_Controller` (`self.GetController`)))
  (`/Game/Blueprints/Enemy/BipedalEnemyAI/Enemy_Controller.TakeDamage` _asenemy_controller DamageAmount HitLocation))

(fn `UserConstructionScript`)