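; Enemy spawner that spawns a requested number of BP_Enemy_Character at random TargetPoints tagged "SpawnPoint", gathered on BeginPlay.
; SpawnEnemies adds to a pending count and loops with random delays between spawns, notifying the GameMode of each enemy and when spawning finishes.
; Room-based logic for waves, door collision and camera blending remains in the graph but is disconnected, with empty events.
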(event `self.ReceiveActorBeginOverlap`
  (params (OtherActor :type "Actor Object Reference"))
  ;[0.6038 1 0.6033] Room Triggers
  ;;[1 1 1] Player Enter Room
)

(event `self.ReceiveActorEndOverlap`
  (params (OtherActor :type "Actor Object Reference"))
  ;[0.6038 1 0.6033] Room Triggers
  ;;[1 1 1] Player Exit Room
)

(event `StartSpawning`
  ;[0.4167 0.4197 1] Spawn Logic
  ;;[1 1 1] Start Spawn
)

(event `SpawnWave`
  ;[0.4167 0.4197 1] Spawn Logic
  ;;[1 1 1] Spawn Wave
)

(event `EnemyWasKilled`
  ;[1 0.2969 0.2969] Enemy Killed
)

(event `self.ReceiveBeginPlay`
  (bind _outactors (`GameplayStatics.GetAllActorsOfClassWithTag` "/Script/Engine.TargetPoint" "SpawnPoint"))
  (set `self.SpawnPoints` _outactors))

(event `SpawnEnemies`
  (params (Amount :type Integer))
  (bind _output_get (set `self.EnemiesLeftToSpawn` (+ Amount (`self.EnemiesLeftToSpawn`))))
  (if (> _output_get 0) :!label _label
    (set `self.IsSpawning` true)
    (`KismetSystemLibrary.Delay` (`KismetMathLibrary.RandomFloatInRange` 1.0 3.0))
    (bind _returnvalue (`|SpawnActorFromClass` "/Game/Blueprints/Enemy/New_Enemy_AI/BP_Enemy_Character.BP_Enemy_Character_C" (`self.GetTransform` (`KismetArrayLibrary.Array_Random` (`self.SpawnPoints`))) "Undefined" "OverrideRootScale" null null))
    (message `/Game/Blueprints/Interfaces/BPI_GameModeInterface.EnemySpawned` (`GameplayStatics.GetGameMode`) _returnvalue)
    (`/Engine/EditorBlueprintResources/StandardMacros.DecrementInt` (`self.EnemiesLeftToSpawn`)
      (:`  `
        (`KismetSystemLibrary.PrintString` "Spawned Enemy")
        (goto _label)))
    (else
      (set `self.IsSpawning` false)
      (`KismetSystemLibrary.PrintString` "Spawn complete")
      (message `/Game/Blueprints/Interfaces/BPI_GameModeInterface.EnemiesFinishedSpawning` (`GameplayStatics.GetGameMode`)))))

(fn `ToggleDoorsActive`
  (params (Activate :type Boolean))
  (for _array_element (`self.Doors`)
    (if Activate
      (`PrimitiveComponent.SetCollisionEnabled` _array_element "QueryAndPhysics")
      (else
        (`PrimitiveComponent.SetCollisionEnabled` _array_element "NoCollision")))))

(fn `UserConstructionScript`)