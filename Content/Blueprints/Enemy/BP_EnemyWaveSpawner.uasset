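; Wave spawner that runs endless rounds of enemies, scaling each round's spawn total by round number.
; A looping timer spawns ground or flying enemies at random TargetPoints tagged SpawnPoint, pausing when the living cap or round quota is reached.
; EnemyKilled resumes the timer mid-wave or starts the next round once all are dead.
; Wave and enemy counters are pushed to BP_TESTHUD.
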(event `self.ReceiveBeginPlay`
  ;[0.97 0.3198 1] INIT
  (`KismetSystemLibrary.Delay` 5.0) ; Do this to avoid weird load level logic breaking stuff
  (bind _outactors (`GameplayStatics.GetAllActorsOfClassWithTag` "/Script/Engine.TargetPoint" "SpawnPoint"))
  (if (`KismetSystemLibrary.IsValid` (`|GetArrayItem` _outactors))
    (set `self.spawnPoints` _outactors)
    (`self.StartNewRound`)
    (else
      (`self.Print` "------------------------- \nCRITICAL ERROR! \nCOULD NOT FIND ANY TARGET POINTS WITH \nActor Tag [SpawnPoint]! \nBP_ENEMYWAVESPAWNER CAN'T FUNCTION \nWITHOUT AT LEAST ONE TARGET POINT MATCHING CRITERIA ABOVE! \n-------------------------" true true (struct :`R` 1.0 :`A` 1.0) 60.0))))

(event `StartNewRound`
  ;[1 1 1] Start New Round
  (`self.Print` "START NEW ROUND" true true (struct :`R` 1.0 :`G` 1.0 :`B` 1.0 :`A` 1.0) 5.0)
  (`/Engine/EditorBlueprintResources/StandardMacros.IncrementInt` (`self.currentRound`)
    (:`  `
      (`self.CalculateTargetSpawnAmount`)
      (`self.UpdateHud`)
      (`KismetSystemLibrary.Delay` (`self.delayBetweenRounds`))
      (`self.StartTimer`))))

(event `StartTimer`
  (bind _enemyspawntimerhandle (`self.enemySpawnTimerHandle`))
  ;[1 1 1] Start Spawn Timer
  (if (`KismetSystemLibrary.K2_IsValidTimerHandle` _enemyspawntimerhandle)
    (`KismetSystemLibrary.Delay` (- (`self.spawnDelay`) (`KismetSystemLibrary.K2_GetTimerRemainingTimeHandle` _enemyspawntimerhandle)))
    (`KismetSystemLibrary.K2_UnPauseTimerHandle` (`self.enemySpawnTimerHandle`))
    (`self.Print` "START TIMER WAS UNPAUSED!" true true (struct :`R` 1.0 :`B` 0.904661 :`A` 1.0) 20.0)
    (else
      (bind _returnvalue (`KismetSystemLibrary.K2_SetTimerDelegate` (delegate `SpawnEnemy`) (`self.spawnDelay`) true))
      (set `self.enemySpawnTimerHandle` _returnvalue)
      (`self.Print` " START TIMER WAS CREATED!" true true (struct :`G` 0.658824 :`B` 1.0 :`A` 1.0) 20.0))))

(event `SpawnEnemy`
  ;[0.6125 1 0.6529] Spawn Enemy
  (if (< (`self.currentLivingEnemies`) (`self.maxLivingEnemies`))
    (if (< (`self.currentEnemiesSpawned`) (`self.maxEnemiesSpawned`))
      (bind _spawnpoint (`self.Get Random Spawn Point`))
      (if (== (`KismetMathLibrary.RandomIntegerInRange` 0 1) 0)
        (bind _returnvalue (`self.GetTransform` _spawnpoint))
        (bind _returnvalue_2 (`|SpawnActorFromClass` "/Game/Blueprints/Enemy/BipedalEnemyAI/BP_Enemy_Character.BP_Enemy_Character_C" _returnvalue "AdjustIfPossibleButDontSpawnIfColliding" "OverrideRootScale" null null))
        (if (`KismetSystemLibrary.IsValid` _returnvalue_2)
          (`self.Print` "ENEMY SPAWNED" true true (struct :`R` 1.0 :`G` 0.343419 :`B` 0.363317 :`A` 1.0) 5.0 :!label _label)
          (`self.UpdateHud`)
          (`/Engine/EditorBlueprintResources/StandardMacros.IncrementInt` (`self.currentLivingEnemies`)
            (:`  `
              (`/Engine/EditorBlueprintResources/StandardMacros.IncrementInt` (`self.currentEnemiesSpawned`)
                (:`  `
                  (if (or (>= (`self.currentEnemiesSpawned`) (`self.maxEnemiesSpawned`)) (>= (`self.currentLivingEnemies`) (`self.maxLivingEnemies`)))
                    (`self.Print` "PAUSE TIMER!" true true (struct :`R` 1.0 :`G` 0.888391 :`A` 1.0) 10.0)
                    (`KismetSystemLibrary.K2_PauseTimerHandle` (`self.enemySpawnTimerHandle`))))))))
        (else
          (bind _returnvalue_3 (`|SpawnActorFromClass` "/Game/Blueprints/Enemy/FlyingEnemyAI/BP_FlyingAI.BP_FlyingAI_C" _returnvalue "AdjustIfPossibleButDontSpawnIfColliding" "OverrideRootScale" null null))
          (if (`KismetSystemLibrary.IsValid` _returnvalue_3)
            (goto _label)))))
    (else
      (`self.Print` "------------ \nWARNING!!! THIS SHOULD NOT TRIGGER!!! \nEnemies at max capacity! \n------------" true true (struct :`R` 1.0 :`G` 0.032916 :`A` 1.0) (`self.spawnDelay`)))))

(event `EnemyKilled`
  ;[1 0.5573 0.5573] Enemy Killed
  (bind _result (`/Engine/EditorBlueprintResources/StandardMacros.DecrementInt` (`self.currentLivingEnemies`))
    (:`  `
      (`KismetSystemLibrary.PrintString` (`KismetStringLibrary.Conv_IntToString` _result))
      (`self.UpdateHud`)
      (if (and (<= (`self.currentLivingEnemies`) 0) (>= (`self.currentEnemiesSpawned`) (`self.maxEnemiesSpawned`)))
        (`KismetSystemLibrary.PrintString` "ROUND OVER!" true true (struct :`R` 1.0 :`B` 0.901108 :`A` 1.0) 4.0)
        (`self.RoundOver`)
        (elif (and (< (`self.currentLivingEnemies`) (`self.maxLivingEnemies`)) (< (`self.currentEnemiesSpawned`) (`self.maxEnemiesSpawned`)) (`KismetSystemLibrary.K2_IsTimerPausedHandle` (`self.enemySpawnTimerHandle`)))
          (`KismetSystemLibrary.PrintString` "START TIMER DURING WAVE" true true (struct :`R` 1.0 :`B` 0.901108 :`A` 1.0) 4.0)
          (`self.StartTimer`))))))

(event `RoundOver`
  ;[1 1 1] Round Over
  (set `self.currentEnemiesSpawned` 0)
  (`self.StartNewRound`))

(fn `CalculateTargetSpawnAmount`
  (set `self.maxEnemiesSpawned` (`KismetMathLibrary.FFloor` (+ 1.0 (* (`self.currentRound`) (`self.SpawnScale`))))))

(fn `Get Random Spawn Point`
  (returns (spawnPoint :type "TargetPoint Object Reference"))
  (if (`KismetSystemLibrary.IsValid` (`KismetArrayLibrary.Array_Random` (`self.spawnPoints`)))
    (bind _outitem (`KismetArrayLibrary.Array_Random` (stale _output_get)))
    (return _outitem)
    (else
      (bind _outactors (`GameplayStatics.GetAllActorsOfClassWithTag` "/Script/Engine.TargetPoint" "SpawnPoint"))
      (bind _output_get (set `self.spawnPoints` _outactors))
      (if (`KismetSystemLibrary.IsValid` _outitem)
        (return _outitem)
        (else
          (`KismetSystemLibrary.PrintString` "CRITICAL ERROR! \nCOULD NOT FIND ANY TARGET POINTS WITH \nActor Tag [SpawnPoint]! \nBP_ENEMYWAVESPAWNER CAN'T FUNCTION \nWITHOUT AT LEAST ONE TARGET POINT MATCHING CRITERIA ABOVE!" true true (struct :`R` 1.0 :`B` 0.094589 :`A` 1.0) 60.0))))))

(fn `Print`
  (params (`In String` :type String) (bPrintToScreen :type Boolean :default true) (bPrintToLog :type Boolean :default true) (TextColor :type "LinearColor Structure" :default (struct :`G` 0.658824 :`B` 1.0 :`A` 1.0)) (Duration :type "Float (single-precision)" :default 4.0) (Key :type Name))
  (`KismetSystemLibrary.PrintString` (`KismetStringLibrary.Concat_StrStr` "[" (`KismetStringLibrary.Conv_DoubleToString` (`KismetSystemLibrary.GetGameTimeInSeconds`)) "] " `In String`) false bPrintToLog TextColor Duration Key))

(fn `UpdateHud`
  (bind _asbp_testhud (cast `/Game/Graphics/Hud/HUDStuff/BP_TESTHUD` (`PlayerController.GetHUD` (`GameplayStatics.GetPlayerController` 0))))
  (`/Game/Graphics/Hud/HUDStuff/TestHUDWidget.UpdateEnemiesCounter` (`/Game/Graphics/Hud/HUDStuff/BP_TESTHUD.HUDRef` _asbp_testhud) (`self.currentLivingEnemies`))
  (bind _hudref (`/Game/Graphics/Hud/HUDStuff/BP_TESTHUD.HUDRef` _asbp_testhud))
  (`/Game/Graphics/Hud/HUDStuff/TestHUDWidget.UpdateWaveCounter` _hudref (`self.currentRound`))
  (`/Game/Graphics/Hud/HUDStuff/TestHUDWidget.UpdateEnemiesToSpawnCount` _hudref (`self.maxEnemiesSpawned`))
  (`/Game/Graphics/Hud/HUDStuff/TestHUDWidget.UpdateTotalEnemiesSpawnedThisRound` _hudref (`self.currentEnemiesSpawned`)))

(fn `UserConstructionScript`)