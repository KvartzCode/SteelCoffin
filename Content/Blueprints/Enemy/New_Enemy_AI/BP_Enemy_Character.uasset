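; Enemy character that runs the Enemy_BT behavior tree when possessed by its AI controller.
; DamageEnemy subtracts health; at zero it sets the blackboard isDead flag, spawns an emitter, notifies the game mode and destroys the actor.
; UpdateWalkSpeed sets the movement component's max walk speed.
; Tick is empty, as the nodes writing player target and distance to the blackboard are disconnected.
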(event `self.ReceivePossessed`
  (params (NewController :type "Controller Object Reference"))
  (`AIController.RunBehaviorTree` (`AIBlueprintHelperLibrary.GetAIController` self) "/Game/Blueprints/Enemy/BehaviorTree/Enemy_BT.Enemy_BT")
  (`KismetSystemLibrary.PrintString` "Heyo"))

(event `self.ReceiveTick`
  (params (DeltaSeconds :type "Float (single-precision)"))
  ;[1 1 1] Sets and constantly updates the CurrentTargetDistance variable in the blackboard to the distance between the enemy and the player
)

(event `/Game/Blueprints/Interfaces/BPI_EnemyInterface.DamageEnemy`
  (params (DamageAmount :type "Float (double-precision)"))
  ;[1 1 1] Enemy Take Damage
  (bind _output_get (set `self.EnemyHealth` (- (`self.EnemyHealth`) DamageAmount)))
  ;[1 1 1] Enemy Death
  (if (<= _output_get 0.0)
    (set `self.isDead` true)
    (`BlackboardComponent.SetValueAsBool` (`AIBlueprintHelperLibrary.GetBlackboard` null) "isDead" true)
    (`GameplayStatics.SpawnEmitterAtLocation` null (`self.K2_GetActorLocation`) (struct) (10.0 10.0 10.0))
    (message `/Game/Blueprints/Interfaces/BPI_GameModeInterface.EnemyKilled` (`GameplayStatics.GetGameMode`) self)
    (`self.K2_DestroyActor`)
    (else
      (`KismetSystemLibrary.PrintString` (`KismetStringLibrary.Conv_DoubleToString` _output_get)))))

(fn `UpdateWalkSpeed`
  (params (NewWalkSpeed :type "Float (double-precision)"))
  (set `CharacterMovementComponent.MaxWalkSpeed` NewWalkSpeed (`self.CharacterMovement`)))

(fn `UserConstructionScript`)