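; Combat room actor that runs waves of BP_EnemyAI and tracks when the room is cleared.
; Child box components tagged "Door" are collected at BeginPlay as collision blockers, initially disabled.
; StartSpawning spawns the first wave at WaveGroups actor transforms; EnemyWasKilled counts down to the next wave or clears the room and disables door collision.
; Overlap events currently do nothing, as the camera blend, door locking and GameMode notification logic is disconnected.
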(event `self.ReceiveBeginPlay`
  ;[0.7792 0.03417 1] INIT
  (for _array_element (`SceneComponent.GetChildrenComponents` (`self.DefaultSceneRoot`) false)
    (if (`ActorComponent.ComponentHasTag` _array_element "Door")
      (bind _asbox_collision (cast `BoxComponent` _array_element))
      (`KismetArrayLibrary.Array_AddUnique` (`self.Doors`) _asbox_collision)))
  (`self.ToggleDoorsActive` false))

(event `self.ReceiveActorBeginOverlap`
  (params (OtherActor :type "Actor Object Reference"))
  ;[0.6038 1 0.6033] Room Triggers
  ;;[1 1 1] Player Enter Room
  (if (`self.RoomCleared`)
    _))

(event `self.ReceiveActorEndOverlap`
  (params (OtherActor :type "Actor Object Reference"))
  ;[0.6038 1 0.6033] Room Triggers
  ;;[1 1 1] Player Exit Room
  (if (`self.RoomCleared`)
    _))

(event `StartSpawning`
  ;[0.4167 0.4197 1] Spawn Logic
  ;;[1 1 1] Start Spawn
  (set `self.WaveCount` 0)
  (`self.SpawnWave`))

(event `SpawnWave`
  (bind _output_wave (break `/Game/Blueprints/TargetPointArray` (`|GetArrayItem` (`self.WaveGroups`) (`self.WaveCount`))))
  ;[0.4167 0.4197 1] Spawn Logic
  ;;[1 1 1] Spawn Wave
  (if (not (`self.RoomCleared`))
    (set `self.EnemyCount` 0)
    (if (not (>= (`self.WaveCount`) (`KismetArrayLibrary.Array_Length` (`self.WaveGroups`))))
      ;;[1 1 1] Spawn enemies
      (for _array_element _output_wave
        (`|SpawnActorFromClass` "/Game/Blueprints/Enemy/BP_EnemyAI.BP_EnemyAI_C" (`self.GetTransform` _array_element) "Undefined" "OverrideRootScale" null null)
        (`/Engine/EditorBlueprintResources/StandardMacros.IncrementInt` (`self.EnemyCount`)))
      (`/Engine/EditorBlueprintResources/StandardMacros.IncrementInt` (`self.WaveCount`)))))

(event `EnemyWasKilled`
  ;[1 0.2969 0.2969] Enemy Killed
  (bind _result (`/Engine/EditorBlueprintResources/StandardMacros.DecrementInt` (`self.EnemyCount`))
    (:`  `
      (if (<= _result 0)
        (if (>= (`self.WaveCount`) (`KismetArrayLibrary.Array_Length` (`self.WaveGroups`)))
          (set `self.RoomCleared` true)
          (`self.ToggleDoorsActive` false)
          (else
            (`self.SpawnWave`)))))))

(fn `ToggleDoorsActive`
  (params (Activate :type Boolean))
  (for _array_element (`self.Doors`)
    (if Activate
      (`PrimitiveComponent.SetCollisionEnabled` _array_element "QueryAndPhysics")
      (else
        (`PrimitiveComponent.SetCollisionEnabled` _array_element "NoCollision")))))

(fn `UserConstructionScript`)