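; Player controller for the mech that sets up Enhanced Input, Health and the HUD, then routes input to the player character.
; Move input drives the legs' movement and rotation, while look input rotates the torso separately.
; Escape and P share one FlipFlop that alternately calls pause and unpause on the Swarm game mode, with leftover debug prints.
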(event `self.ReceiveBeginPlay`
  (bind _returnvalue (subsystem `EnhancedInputLocalPlayerSubsystem`))
  ;[1 1 1] INIT
  (`/Engine/EditorBlueprintResources/StandardMacros.IsValid` _returnvalue
    (:`Is Valid`
      (`EnhancedInputSubsystemInterface.AddMappingContext` _returnvalue "/Game/Input/IMC_TankInput.IMC_TankInput" 0 (struct))
      (bind _asbpc_player_mech_character (cast `/Game/Blueprints/BPC_PlayerMechCharacter` (`GameplayStatics.GetPlayerCharacter` 0)))
      (set `self.playerCharacter_ref` _asbpc_player_mech_character)
      (set `self.Health` (`self.MaxHealth`))
      (bind _returnvalue_2 (`|CreateWidget` "/Game/Blueprints/WBP_HUD.WBP_HUD_C"))
      (`UserWidget.AddToViewport` _returnvalue_2 0))))

(event `Key|Escape` :paused true
  (params (Key :type "Key Structure"))
  ;[1 1 1] Pause Input
  (:`Pressed`
    (`/Engine/EditorBlueprintResources/StandardMacros.FlipFlop` :!label _label
      (:`A`
        (`KismetSystemLibrary.PrintString` "Hello")
        (bind _asgm_swarm (cast `/Game/Blueprints/GM_Swarm` (`GameplayStatics.GetGameMode`)))
        (`/Game/Blueprints/GM_Swarm.PauseGame` _asgm_swarm))
      (:`B`
        (`KismetSystemLibrary.PrintString` "Hello")
        (bind _asgm_swarm_2 (cast `/Game/Blueprints/GM_Swarm` (`GameplayStatics.GetGameMode`)))
        (`/Game/Blueprints/GM_Swarm.UnPauseGame` _asgm_swarm_2)))))

(event `Key|P` :paused true
  (params (Key :type "Key Structure"))
  ;[1 1 1] Pause Input
  (:`Pressed`
    (goto _label)))

(event `EnhancedInput|/Game/Input/IA_Move`
  (params (ActionValue :type "Vector2D Structure") (ElapsedSeconds :type "Float (double-precision)") (TriggeredSeconds :type "Float (double-precision)") (InputAction :type "InputAction Object Reference" :default "/Game/Input/IA_Move.IA_Move"))
  (:`Triggered`
    (`/Game/Blueprints/BPC_PlayerMechCharacter.MoveLegs` (`self.playerCharacter_ref`) ActionValue_Y)
    (`/Game/Blueprints/BPC_PlayerMechCharacter.RotateLegs` (`self.playerCharacter_ref`) ActionValue_X)))

(event `EnhancedInput|/Game/Input/IA_Look`
  (params (ActionValue :type "Vector2D Structure") (ElapsedSeconds :type "Float (double-precision)") (TriggeredSeconds :type "Float (double-precision)") (InputAction :type "InputAction Object Reference" :default "/Game/Input/IA_Look.IA_Look"))
  (:`Triggered`
    (`/Game/Blueprints/BPC_PlayerMechCharacter.RotateTorso` (`self.playerCharacter_ref`) ActionValue)))

(fn `UserConstructionScript`)