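; Player controller for the mech that handles player input and owns the player's health.
; Enhanced Input actions forward walk, leg, torso and camera messages to the character and toggle sprinting on BP_PlayerMech.
; Escape or P flip-flops pause through GM_Swarm.
; Damage triggers a camera shake and notifies the game mode at zero health, while heat logic is disconnected and GetHeat returns zeros.
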(event `self.ReceiveBeginPlay`
  (bind _returnvalue (subsystem `EnhancedInputLocalPlayerSubsystem`))
  ;[1 1 1] INIT
  (`/Engine/EditorBlueprintResources/StandardMacros.IsValid` _returnvalue
    (:`Is Valid`
      (`EnhancedInputSubsystemInterface.AddMappingContext` _returnvalue "/Game/Blueprints/Input/IMC_TankInput.IMC_TankInput" 0 (struct))
      (set `self.playerCharacter_ref` (`GameplayStatics.GetPlayerCharacter` 0))
      (set `self.Health` (`self.MaxHealth`))
      (bind _asbp_player_mech (cast `/Game/Blueprints/Player/BP_PlayerMech` (`GameplayStatics.GetPlayerCharacter` 0)))
      (set `self.SpecificPlayerCharRef` _asbp_player_mech))))

(event `Key|Escape` :paused true
  (params (Key :type "Key Structure"))
  ;[1 1 1] Pause Input
  ;;[1 1 1] TODO: Replace with Input Action
  (:`Pressed`
    (`/Engine/EditorBlueprintResources/StandardMacros.FlipFlop` :!label _label
      (:`A`
        (`KismetSystemLibrary.PrintString` "Hello")
        (bind _asgm_swarm (cast `/Game/Blueprints/GameModes/GM_Swarm` (`GameplayStatics.GetGameMode`)))
        (`/Game/Blueprints/GameModes/GM_Swarm.PauseGame` _asgm_swarm))
      (:`B`
        (`KismetSystemLibrary.PrintString` "Hello")
        (bind _asgm_swarm_2 (cast `/Game/Blueprints/GameModes/GM_Swarm` (`GameplayStatics.GetGameMode`)))
        (`/Game/Blueprints/GameModes/GM_Swarm.UnPauseGame` _asgm_swarm_2)))))

(event `Key|P` :paused true
  (params (Key :type "Key Structure"))
  ;[1 1 1] Pause Input
  ;;[1 1 1] TODO: Replace with Input Action
  (:`Pressed`
    (goto _label)))

(event `EnhancedInput|/Game/Blueprints/Input/TankInput/IA_Move`
  (params (ActionValue :type "Vector2D Structure") (ElapsedSeconds :type "Float (double-precision)") (TriggeredSeconds :type "Float (double-precision)") (InputAction :type "InputAction Object Reference" :default "/Game/Blueprints/Input/TankInput/IA_Move.IA_Move"))
  ;[1 1 1] Movement
  (:`Triggered`
    (message `/Game/Blueprints/Interfaces/BPI_PlayerCharacter.Walk` (`self.playerCharacter_ref`) ActionValue_X)))

(event `EnhancedInput|/Game/Blueprints/Input/TankInput/IA_Rotate`
  (params (ActionValue :type "Float (double-precision)") (ElapsedSeconds :type "Float (double-precision)") (TriggeredSeconds :type "Float (double-precision)") (InputAction :type "InputAction Object Reference" :default "/Game/Blueprints/Input/TankInput/IA_Rotate.IA_Rotate"))
  ;[1 1 1] Movement
  (:`Triggered`
    (message `/Game/Blueprints/Interfaces/BPI_PlayerCharacter.RotateLegs` (`self.playerCharacter_ref`) ActionValue)))

(event `EnhancedInput|/Game/Blueprints/Input/TankInput/IA_Look`
  (params (ActionValue :type "Vector2D Structure") (ElapsedSeconds :type "Float (double-precision)") (TriggeredSeconds :type "Float (double-precision)") (InputAction :type "InputAction Object Reference" :default "/Game/Blueprints/Input/TankInput/IA_Look.IA_Look"))
  ;[1 1 1] Movement
  (:`Triggered`
    (message `/Game/Blueprints/Interfaces/BPI_PlayerCharacter.RotateTorso` (`self.playerCharacter_ref`) ActionValue_X)
    (message `/Game/Blueprints/Interfaces/BPI_PlayerCharacter.RotateCamera` (`self.playerCharacter_ref`) 0.0 ActionValue_Y)))

(event `EnhancedInput|/Game/Blueprints/Input/TankInput/IA_Sprint`
  (params (ActionValue :type Boolean) (ElapsedSeconds :type "Float (double-precision)") (TriggeredSeconds :type "Float (double-precision)") (InputAction :type "InputAction Object Reference" :default "/Game/Blueprints/Input/TankInput/IA_Sprint.IA_Sprint"))
  ;[1 1 1] Movement
  (:`Triggered`
    (set `/Game/Blueprints/Player/BP_PlayerMech.isSprinting` true (`self.SpecificPlayerCharRef`)))
  (:`Started`
    (`KismetSystemLibrary.PrintString` "STARTED PRESSING"))
  (:`Completed`
    (set `/Game/Blueprints/Player/BP_PlayerMech.isSprinting` false (`self.SpecificPlayerCharRef`))
    (`KismetSystemLibrary.PrintString` "stopped  PRESSING")))

(event `/Game/Blueprints/Interfaces/BPI_PlayerControllerInterface.HealPlayer`
  (params (healValue :type Integer))
  ;[0.3286 1 0.4401] Player Health
  (set `self.Health` (+ (`self.Health`) healValue)))

(event `/Game/Blueprints/Interfaces/BPI_PlayerControllerInterface.DamagePlayer`
  (params (damage :type Integer))
  ;[0.3286 1 0.4401] Player Health
  (bind _output_get (set `self.Health` (- (`self.Health`) damage)))
  (`GameplayStatics.PlayWorldCameraShake` "/Game/Blueprints/Player/BP_DamageCameraShake.BP_DamageCameraShake_C" (`SceneComponent.K2_GetComponentLocation` (`Character.Mesh` (`GameplayStatics.GetPlayerCharacter` 0))) 0.0 5000.0 0.0)
  (if (<= _output_get 0)
    (message `/Game/Blueprints/Interfaces/BPI_GameModeInterface.PlayerDied` (`GameplayStatics.GetGameMode`) 0)))

(fn `GetHealth`
  (returns (CurrentHealth :type Integer) (MaxHealth :type Integer))
  (return (`self.Health`) (`self.MaxHealth`)))

(fn `GetHeat`
  (returns (CurrentHeat :type "Float (double-precision)") (MaxHeat :type "Float (double-precision)"))
  (return 0.0 0.0))

(fn `UserConstructionScript`)