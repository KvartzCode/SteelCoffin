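; Player mech with independently rotating legs and torso, leg-relative walking, a pitch-clamped camera and two autocannons.
; Tick traces from the camera to aim both weapons, then runs each one's cooldown check, firing while its FlipFlop-toggled input flag is set.
; Shots are muzzle line traces with sound and shell effects, sending damage messages to actors tagged EnemyMech.
; Manual-fire events and target marking/range logic are leftovers, unused or disconnected.
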(event `self.ReceiveBeginPlay`
  (bind _acan_firerate (`self.Acan_FireRate`))
  ;[0.02122 0 0.4072] INIT
  ;;[1 1 1] ACAN STATS INIT
  (set `self.F_LeftWeaponTotalCooldown` _acan_firerate)
  (set `self.F_RightWeaponTotalCooldown` _acan_firerate))

(event `Key|F`
  (params (Key :type "Key Structure"))
  ;[1 1 1] Targeting
  ;;[1 1 1] Manual Targeting Increase distance
)

(event `EnhancedInput|/Game/Blueprints/Input/TankInput/IA_ShootLeft`
  (params (ActionValue :type Boolean) (ElapsedSeconds :type "Float (double-precision)") (TriggeredSeconds :type "Float (double-precision)") (InputAction :type "InputAction Object Reference" :default "/Game/Blueprints/Input/TankInput/IA_ShootLeft.IA_ShootLeft"))
  ;[1 1 1] Fire
  ;;[1 1 1] Mouse Buttons
  (:`Triggered`
    (`/Engine/EditorBlueprintResources/StandardMacros.FlipFlop`
      (:`A`
        (set `self.B_LeftMousePressed` true))
      (:`B`
        (set `self.B_LeftMousePressed` false)))))

(event `CE_FireLeftWeapon_AUTO`
  (bind _leftweapon (`self.LeftWeapon`))
  (bind _returnvalue (`SceneComponent.GetSocketLocation` (`self.LeftWeapon`) "Muzzle"))
  (bind (_returnvalue_roll _returnvalue_pitch _returnvalue_yaw) (`KismetMathLibrary.BreakRotator` (`SceneComponent.K2_GetComponentRotation` _leftweapon)))
  ;[1 1 1] Fire
  ;;[1 1 1] AutoFire
  (set `self.B_LeftWeaponFireReady` false)
  (set `self.F_LeftWeaponCurrentCooldown` (`self.F_LeftWeaponTotalCooldown`))
  (bind (_outhit _returnvalue_2) (`KismetSystemLibrary.LineTraceSingle` :`Start` _returnvalue :`End` (+ _returnvalue (* (`KismetMathLibrary.GetDirectionUnitVector` _returnvalue (`self.Location`)) (`KismetMathLibrary.Conv_DoubleToVector` 30000.0))) :`TraceChannel` "TraceTypeQuery2" :`DrawDebugType` "ForDuration" :`TraceColor` (struct :`G` 1.0 :`B` 0.246827 :`A` 0.393) :`TraceHitColor` (struct :`R` 0.964683 :`G` 0.046352 :`B` 1.0 :`A` 1.0) :`DrawTime` 3.0))
  (`self.Handle Hit Enemy` _outhit _returnvalue_2)
  (`GameplayStatics.PlaySoundAtLocation` "/Game/Sounds/Mech/Weapons/Akan40mm/40mmFire.40mmFire" (`SceneComponent.K2_GetComponentLocation` _leftweapon) (struct) 1.0 1.0 0.0 null null null null)
  (`NiagaraFunctionLibrary.SpawnSystemAtLocation` "/Game/Graphics/Effects/FX_ShellDrop.FX_ShellDrop" (`SceneComponent.K2_GetComponentLocation` (`self.LeftWeapon`)) (`KismetMathLibrary.MakeRotator` _returnvalue_roll _returnvalue_pitch (+ _returnvalue_yaw 180.0))))

(event `Key|MouseScrollUp`
  (params (Key :type "Key Structure"))
  ;[1 1 1] Targeting
  ;;[1 1 1] Manual Targeting Increase distance
)

(event `EnhancedInput|/Game/Blueprints/Input/TankInput/IA_ShootRight`
  (params (ActionValue :type Boolean) (ElapsedSeconds :type "Float (double-precision)") (TriggeredSeconds :type "Float (double-precision)") (InputAction :type "InputAction Object Reference" :default "/Game/Blueprints/Input/TankInput/IA_ShootRight.IA_ShootRight"))
  ;[1 1 1] Fire
  ;;[1 1 1] Mouse Buttons
  (:`Triggered`
    (`/Engine/EditorBlueprintResources/StandardMacros.FlipFlop`
      (:`A`
        (set `self.B_RightMousePressed` true))
      (:`B`
        (set `self.B_RightMousePressed` false)))))

(event `CE_FireRightWeapon_AUTO`
  (bind _rightweapon (`self.RightWeapon`))
  (bind _returnvalue (`SceneComponent.GetSocketLocation` (`self.RightWeapon`) "Muzzle"))
  ;[1 1 1] Fire
  ;;[1 1 1] AutoFire
  (set `self.B_RightWeaponFireReady` false)
  (set `self.F_RightWeaponCurrentCooldown` (`self.F_RightWeaponTotalCooldown`))
  (bind (_outhit _returnvalue_2) (`KismetSystemLibrary.LineTraceSingle` :`Start` _returnvalue :`End` (+ _returnvalue (* (`KismetMathLibrary.GetDirectionUnitVector` _returnvalue (`self.Location`)) (`KismetMathLibrary.Conv_DoubleToVector` 30000.0))) :`TraceChannel` "TraceTypeQuery2" :`DrawDebugType` "ForDuration" :`TraceColor` (struct :`G` 1.0 :`B` 0.247059 :`A` 0.392157) :`TraceHitColor` (struct :`R` 0.964683 :`G` 0.046352 :`B` 1.0 :`A` 1.0) :`DrawTime` 3.0))
  (`self.Handle Hit Enemy` _outhit _returnvalue_2)
  (`GameplayStatics.PlaySoundAtLocation` "/Game/Sounds/Mech/Weapons/Akan40mm/40mmFire.40mmFire" (`SceneComponent.K2_GetComponentLocation` (`self.RightWeapon`)) (struct) 1.0 1.0 0.0 null null null null)
  (`NiagaraFunctionLibrary.SpawnSystemAtLocation` "/Game/Graphics/Effects/FX_ShellDrop.FX_ShellDrop" (`SceneComponent.K2_GetComponentLocation` _rightweapon) (`SceneComponent.K2_GetComponentRotation` _rightweapon)))

(event `self.ReceiveTick`
  (params (DeltaSeconds :type "Float (single-precision)"))
  (bind _camera (`self.Camera`))
  (bind _leftweapon (`self.LeftWeapon`))
  (bind _rightweapon (`self.RightWeapon`))
  (bind _leftweapon_2 (`self.LeftWeapon`))
  (bind _rightweapon_2 (`self.RightWeapon`))
  (bind _returnvalue (`SceneComponent.K2_GetComponentLocation` _camera))
  (bind _returnvalue_2 (+ _returnvalue (* (`SceneComponent.GetForwardVector` _camera) (`KismetMathLibrary.Conv_DoubleToVector` 30000.0))))
  (bind (_outhit _returnvalue_3) (`KismetSystemLibrary.LineTraceSingle` :`Start` _returnvalue :`End` _returnvalue_2 :`TraceChannel` "TraceTypeQuery2" :`TraceColor` (struct :`R` 1.0 :`A` 0.393) :`TraceHitColor` (struct :`R` 0.964683 :`G` 0.046352 :`B` 1.0 :`A` 1.0) :`DrawTime` 0.5))
  (if _returnvalue_3
    (bind (_bblockinghit _binitialoverlap _time _distance _location) (`GameplayStatics.BreakHitResult` _outhit))
    (`SceneComponent.K2_SetWorldRotation` _leftweapon_2 (`KismetMathLibrary.FindLookAtRotation` (`SceneComponent.K2_GetComponentLocation` _leftweapon_2) _location) false false)
    (`SceneComponent.K2_SetWorldRotation` _rightweapon_2 (`KismetMathLibrary.FindLookAtRotation` (`SceneComponent.K2_GetComponentLocation` _rightweapon_2) _location) false false)
    (set `self.Location` _location)
    (else
      (`SceneComponent.K2_SetWorldRotation` _leftweapon (`KismetMathLibrary.FindLookAtRotation` (`SceneComponent.K2_GetComponentLocation` _leftweapon) _returnvalue_2) false false)
      (`SceneComponent.K2_SetWorldRotation` _rightweapon (`KismetMathLibrary.FindLookAtRotation` (`SceneComponent.K2_GetComponentLocation` _rightweapon) _returnvalue_2) false false)
      (set `self.Location` _returnvalue_2)))
  ;[0.1231 1 0.2507] Comment
  (`self.CE_WeaponLeftFireCheck` DeltaSeconds)
  (`self.CE_WeaponRightFireCheck` DeltaSeconds))

(event `Key|MouseScrollDown`
  (params (Key :type "Key Structure"))
  ;[1 1 1] Targeting
  ;;[1 1 1] Manual Targeting Increase distance
)

(event `CE_WeaponLeftFireCheck`
  (params (deltaTime :type "Float (double-precision)"))
  ;[0.1231 1 0.2507] Comment
  (if (`self.B_LeftWeaponFireReady`)
    (if (`self.B_LeftMousePressed`)
      (if (`self.AutoTargeting_enabled`)
        _
        (else
          _))
      (`self.CE_FireLeftWeapon_AUTO`))
    (else
      (bind _output_get (set `self.F_LeftWeaponCurrentCooldown` (- (`self.F_LeftWeaponCurrentCooldown`) deltaTime)))
      (if (< _output_get 0.0)
        (set `self.B_LeftWeaponFireReady` true)))))

(event `CE_FireLeftWeapon_MANUAL`
  (bind _leftweapon (`self.LeftWeapon`))
  ;[1 1 1] Fire
  ;;[1 0 0 1 40] Deprecated
  (set `self.B_LeftWeaponFireReady` false)
  (set `self.F_LeftWeaponCurrentCooldown` (`self.F_LeftWeaponTotalCooldown`))
  (`GameplayStatics.PlaySoundAtLocation` "/Game/Sounds/Mech/Weapons/Akan40mm/40mmFire.40mmFire" (`SceneComponent.K2_GetComponentLocation` (`self.LeftWeapon`)) (struct) 1.0 1.0 0.0 null null null null)
  (bind (_outhit _returnvalue) (`KismetSystemLibrary.LineTraceSingle` :`Start` (`SceneComponent.K2_GetComponentLocation` _leftweapon) :`End` (`SceneComponent.K2_GetComponentLocation` _leftweapon) :`TraceChannel` "TraceTypeQuery2" :`DrawDebugType` "ForDuration" :`TraceColor` (struct :`R` 0.033676 :`G` 1.0 :`A` 1.0) :`DrawTime` 20.0))
  (`self.Handle Hit Enemy` _outhit _returnvalue))

(event `CE_WeaponRightFireCheck`
  (params (deltaTime :type "Float (double-precision)"))
  ;[0.1231 1 0.2507] Comment
  (if (`self.B_RightWeaponFireReady`)
    (if (`self.B_RightMousePressed`)
      (if (`self.AutoTargeting_enabled`)
        _
        (else
          _))
      (`self.CE_FireRightWeapon_AUTO`))
    (else
      (bind _output_get (set `self.F_RightWeaponCurrentCooldown` (- (`self.F_RightWeaponCurrentCooldown`) deltaTime)))
      (if (< _output_get 0.0)
        (set `self.B_RightWeaponFireReady` true)))))

(event `CE_FireRightWeapon_MANUAL`
  (bind _rightweapon (`self.RightWeapon`))
  ;[1 1 1] Fire
  ;;[1 0 0 1 40] Deprecated
  (set `self.B_RightWeaponFireReady` false)
  (set `self.F_RightWeaponCurrentCooldown` (`self.F_RightWeaponTotalCooldown`))
  (`GameplayStatics.PlaySoundAtLocation` "/Game/Sounds/Mech/Weapons/Akan40mm/40mmFire.40mmFire" (`SceneComponent.K2_GetComponentLocation` (`self.RightWeapon`)) (struct) 1.0 1.0 0.0 null null null null)
  (bind (_outhit _returnvalue) (`KismetSystemLibrary.LineTraceSingle` :`Start` (`SceneComponent.K2_GetComponentLocation` _rightweapon) :`End` (`SceneComponent.K2_GetComponentLocation` _rightweapon) :`TraceChannel` "TraceTypeQuery2" :`DrawDebugType` "ForDuration" :`TraceColor` (struct :`R` 0.033676 :`G` 1.0 :`A` 1.0) :`DrawTime` 20.0))
  (`self.Handle Hit Enemy` _outhit _returnvalue))

(event `Key|E`
  (params (Key :type "Key Structure"))
  ;[1 1 1] Targeting
  ;;[1 1 1] Automatic targeting
)

(event `/Game/Blueprints/Interfaces/BPI_PlayerCharacter.Walk`
  (params (Direction :type "Float (double-precision)"))
  (bind (_returnvalue_x _returnvalue_y) (`KismetMathLibrary.BreakVector` (`SceneComponent.GetForwardVector` (`self.Legs`))))
  (`self.AddMovementInput` (`KismetMathLibrary.MakeVector` _returnvalue_x _returnvalue_y) (* Direction (`self.LegMoveSpeed`))))

(event `/Game/Blueprints/Interfaces/BPI_PlayerCharacter.RotateLegs`
  (params (Direction :type "Float (double-precision)"))
  (`SceneComponent.K2_SetWorldRotation` (`self.Legs`) (`KismetMathLibrary.MakeRotator` (.roll (`SceneComponent.K2_GetComponentRotation` (`self.Legs`))) (.pitch (`SceneComponent.K2_GetComponentRotation` (`self.Legs`))) (+ (.yaw (`SceneComponent.K2_GetComponentRotation` (`self.Legs`))) Direction)) false false))

(event `/Game/Blueprints/Interfaces/BPI_PlayerCharacter.RotateTorso`
  (params (Direction :type "Float (double-precision)"))
  (`SceneComponent.K2_SetWorldRotation` (`self.Torso`) (`KismetMathLibrary.MakeRotator` (.roll (`SceneComponent.K2_GetComponentRotation` (`self.Torso`))) (.pitch (`SceneComponent.K2_GetComponentRotation` (`self.Torso`))) (+ (.yaw (`SceneComponent.K2_GetComponentRotation` (`self.Torso`))) Direction)) false false))

(event `/Game/Blueprints/Interfaces/BPI_PlayerCharacter.RotateCamera`
  (params (X :type "Float (double-precision)") (Y :type "Float (double-precision)"))
  (bind _returnvalue (`KismetMathLibrary.MakeRotator` 0.0 (* Y -2.5)))
  (bind (_returnvalue_roll _returnvalue_pitch) (`KismetMathLibrary.BreakRotator` (`SceneComponent.K2_GetComponentRotation` (`self.SpringArm`))))
  (bind _returnvalue_2 (+ _returnvalue_pitch (.pitch _returnvalue)))
  (if (and (< _returnvalue_2 (`self.CameraMaxRotation`)) (> _returnvalue_2 (`self.CameraMinRotation`)))
    (`SceneComponent.K2_AddLocalRotation` (`self.SpringArm`) _returnvalue false false)))

(fn `Handle Hit Enemy`
  (params (OutHit :type "HitResult Structure (by ref)") (DidLineHitAnything :type Boolean))
  (bind (_bblockinghit _binitialoverlap _time _distance _location _impactpoint _normal _impactnormal _physmat _hitactor) (`GameplayStatics.BreakHitResult` OutHit))
  (if DidLineHitAnything
    (if (`self.ActorHasTag` _hitactor "EnemyMech")
      (message `/Game/Blueprints/Interfaces/BPI_EnemyInterface.DamageEnemy` _hitactor (`self.Acan_Damage`) _location)))
  (return))

(fn `UserConstructionScript`)