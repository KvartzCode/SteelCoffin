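; Player mech character with independently turning legs and torso, sprinting with an FOV kick, and two autofire guns.
; Tick traces from the camera to aim both guns, then runs per-gun cooldown checks on mouse-toggled fire flags.
; Shots are hitscan traces dispatching damage and effects by actor tag, sharing a heat pool with overheat lockout.
; Capsule overlap damages small destructibles; older manual-fire and targeting logic remains unused.
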(event `self.ReceiveBeginPlay`
  (bind _acan_firerate (`self.Acan_FireRate`))
  ;[0.4072 0.05874 0.3982] INIT
  ;;[1 1 1] ACAN STATS INIT
  (set `self.LeftWeaponTotalCooldown` _acan_firerate)
  (set `self.RightWeaponTotalCooldown` (* _acan_firerate 0.25)))

(event `self.ReceiveTick`
  (params (DeltaSeconds :type "Float (single-precision)"))
  (bind _camera (`self.Camera`))
  (bind _charactermovement (`self.CharacterMovement`))
  (bind _returnvalue (`SceneComponent.K2_GetComponentLocation` _camera))
  (bind _returnvalue_2 (+ _returnvalue (* (`SceneComponent.GetForwardVector` _camera) (`self.WeaponRange`))))
  ;[0.4423 0.4684 1] Aim Weapons to Camera look direction
  (`KismetSystemLibrary.FlushPersistentDebugLines`)
  (bind (_outhit _returnvalue_3) (`KismetSystemLibrary.LineTraceSingle` :`Start` _returnvalue :`End` _returnvalue_2 :`TraceChannel` "TraceTypeQuery2" :`TraceColor` (struct :`R` 1.0 :`A` 0.393) :`TraceHitColor` (struct :`R` 0.964683 :`G` 0.046352 :`B` 1.0 :`A` 1.0) :`DrawTime` 0.0))
  (if _returnvalue_3
    (`self.AimWeapons` (`.Location` (`GameplayStatics.BreakHitResult` _outhit)))
    (else
      (`self.AimWeapons` _returnvalue_2)))
  (`self.CE_WeaponLeftFireCheck` DeltaSeconds)
  (`self.CE_WeaponRightFireCheck` DeltaSeconds)
  (`|ExecutionSequence`
    (:`then_0`
      ;[1 1 1] Sprinting
      (if (`self.isSprinting`)
        (if (not (== (`CameraComponent.FieldOfView` (`self.Camera`)) 100.0))
          (`/Engine/EditorBlueprintResources/StandardMacros.DoOnce` false :!label _label
            (:`Completed`
              (bind (_direction _lerptrack) (`Timeline|Timeline` :!via `PlayFromStart` :!label _label_2)
                (:`Update`
                  (`CameraComponent.SetFieldOfView` (`self.Camera`) (`KismetMathLibrary.Lerp` 90.0 100.0 _lerptrack))
                  (if (`self.isSprinting`)
                    (set `CharacterMovementComponent.MaxWalkSpeed` 2600.0 _charactermovement)
                    (else
                      (set `CharacterMovementComponent.MaxWalkSpeed` 1700.0 _charactermovement))))))))
        (elif (not (== (`CameraComponent.FieldOfView` (`self.Camera`)) 90.0))
          (`|ExecutionSequence`
            (:`then_0`
              (goto _label :!via `Reset`))
            (:`then_1`
              (goto _label_2 :!via `Reverse`))))))
    (:`then_1`
      ;[1 1 1] Heat go down while not shooting
      (if (<= (`self.HeatDownCooldown`) 0.0)
        (if (> (`self.CurrentHeat`) 0.0)
          (set `self.CurrentHeat` (- (`self.CurrentHeat`) (* DeltaSeconds 32.0))))))))

(event `CE_FireLeftWeapon_AUTO`
  ;[1 0.08854 0.08854] Shoot Logic
  ;;[1 1 1] AutoFire
  (`self.CheckHeat` 1.25
    (:`Fire`
      (set `self.LeftWeaponFireReady` false)
      (set `self.LeftWeaponCurrentCooldown` (`self.LeftWeaponTotalCooldown`))
      (`self.HandleAutoFireLogic` (`self.LeftWeapon`))
      (`SkeletalMeshComponent.PlayAnimation` (`self.WL_GunBarrel`) "/Game/Graphics/Player/Weapons/WeaponAnim/WL_FireAnim.WL_FireAnim" false)
      (if (>= (`self.CurrentHeat`) (`self.MaxHeat`)) :!label _label_3
        (`KismetSystemLibrary.Delay` 3.0)
        (set `self.CurrentHeat` 0.0)
        (set `self.Overheated` false)))))

(event `EnhancedInput|/Game/Blueprints/Input/TankInput/IA_ShootLeft`
  (params (ActionValue :type Boolean) (ElapsedSeconds :type "Float (double-precision)") (TriggeredSeconds :type "Float (double-precision)") (InputAction :type "InputAction Object Reference" :default "/Game/Blueprints/Input/TankInput/IA_ShootLeft.IA_ShootLeft"))
  ;[1 0.08854 0.08854] Shoot Logic
  ;;[1 1 1] Mouse Buttons
  (:`Triggered`
    (`/Engine/EditorBlueprintResources/StandardMacros.FlipFlop`
      (:`A`
        (set `self.LeftMousePressed` true))
      (:`B`
        (set `self.LeftMousePressed` false)))))

(event `CE_FireRightWeapon_AUTO`
  ;[1 0.08854 0.08854] Shoot Logic
  ;;[1 1 1] AutoFire
  (`self.CheckHeat` 0.45
    (:`Fire`
      (set `self.RightWeaponFireReady` false)
      (set `self.RightWeaponCurrentCooldown` (`self.RightWeaponTotalCooldown`))
      (`self.HandleAutoFireLogic` (`self.RightWeapon`) true)
      (`SkeletalMeshComponent.PlayAnimation` (`self.WR_GunBarrel`) "/Game/Graphics/Player/Weapons/WeaponAnim/WR_FireAnim.WR_FireAnim" false)
      (goto _label_3))))

(event `EnhancedInput|/Game/Blueprints/Input/TankInput/IA_ShootRight`
  (params (ActionValue :type Boolean) (ElapsedSeconds :type "Float (double-precision)") (TriggeredSeconds :type "Float (double-precision)") (InputAction :type "InputAction Object Reference" :default "/Game/Blueprints/Input/TankInput/IA_ShootRight.IA_ShootRight"))
  ;[1 0.08854 0.08854] Shoot Logic
  ;;[1 1 1] Mouse Buttons
  (:`Triggered`
    (`/Engine/EditorBlueprintResources/StandardMacros.FlipFlop`
      (:`A`
        (set `self.RightMousePressed` true))
      (:`B`
        (set `self.RightMousePressed` false)))))

(event `CE_FireLeftWeapon_MANUAL`
  ;[1 0 0 1 40] Deprecated
)

(event `CE_FireRightWeapon_MANUAL`
  ;[1 0 0 1 40] Deprecated
)

(event `CE_WeaponLeftFireCheck`
  (params (deltaTime :type "Float (double-precision)"))
  ;[1 0.08854 0.08854] Shoot Logic
  ;;[1 1 1] Check if can shoot
  (if (`self.LeftWeaponFireReady`)
    (if (`self.LeftMousePressed`)
      (if (`self.AutoTargeting_enabled`)
        _
        (else
          _))
      (`self.CE_FireLeftWeapon_AUTO`)
      (set `self.HeatDownCooldown` 5.0 :!label _label_4)
      (else
        (set `self.HeatDownCooldown` (- (`self.HeatDownCooldown`) deltaTime) :!label _label_5)))
    (else
      (bind _output_get (set `self.LeftWeaponCurrentCooldown` (- (`self.LeftWeaponCurrentCooldown`) deltaTime)))
      (if (< _output_get 0.0)
        (set `self.LeftWeaponFireReady` true)))))

(event `CE_WeaponRightFireCheck`
  (params (deltaTime :type "Float (double-precision)"))
  ;[1 0.08854 0.08854] Shoot Logic
  ;;[1 1 1] Check if can shoot
  (if (`self.RightWeaponFireReady`)
    (if (`self.RightMousePressed`)
      (if (`self.AutoTargeting_enabled`)
        _
        (else
          _))
      (`self.CE_FireRightWeapon_AUTO`)
      (goto _label_4)
      (else
        (goto _label_5)))
    (else
      (bind _output_get (set `self.RightWeaponCurrentCooldown` (- (`self.RightWeaponCurrentCooldown`) deltaTime)))
      (if (< _output_get 0.0)
        (set `self.RightWeaponFireReady` true)))))

(event `/Game/Blueprints/Interfaces/BPI_PlayerCharacter.Walk`
  (params (Direction :type "Float (double-precision)"))
  (bind _returnvalue (`KismetMathLibrary.SignOfFloat` Direction))
  (bind (_returnvalue_x _returnvalue_y) (`KismetMathLibrary.BreakVector` (* (* (`SceneComponent.GetRightVector` (`self.Mesh`)) 9999.0) -1.0)))
  ;[1 0.9979 0.3372] Movement
  (if (> _returnvalue 0.0)
    (set `self.isWalkingBack` false)
    (else
      (set `self.isWalkingBack` true)))
  (`self.AddMovementInput` (`KismetMathLibrary.MakeVector` _returnvalue_x _returnvalue_y) (* (* _returnvalue (`self.LegMoveSpeed`)) (`GameplayStatics.GetWorldDeltaSeconds`))))

(event `/Game/Blueprints/Interfaces/BPI_PlayerCharacter.RotateLegs`
  (params (Direction :type "Float (double-precision)"))
  (bind _returnvalue (`SceneComponent.GetRelativeTransform` (`self.Torso`)))
  (bind _returnvalue_2 (`KismetMathLibrary.MakeRotator` 0.0 0.0 (* (* Direction (`self.LegRotationSpeed`)) (`GameplayStatics.GetWorldDeltaSeconds`))))
  ;[1 0.9979 0.3372] Movement
  (set `self.TurnDirection` Direction)
  (`SceneComponent.K2_AddLocalRotation` (`self.Mesh`) _returnvalue_2 false false)
  (`SceneComponent.K2_AddLocalRotation` (`self.Torso`) (* _returnvalue_2 -1.0) false false)
  (if (or (>= (.yaw (.rotation _returnvalue)) 90.0) (< (.yaw (.rotation _returnvalue)) -90.0))
    (`SceneComponent.K2_AddLocalRotation` (`self.Torso`) _returnvalue_2 false false)))

(event `Key|F`
  (params (Key :type "Key Structure"))
  ;[1 0 0 1 40] Deprecated
  ;;[1 1 1] Targeting
  ;;;[1 1 1] Manual Targeting Increase distance
)

(event `Key|MouseScrollUp`
  (params (Key :type "Key Structure"))
  ;[1 0 0 1 40] Deprecated
  ;;[1 1 1] Targeting
  ;;;[1 1 1] Manual Targeting Increase distance
)

(event `/Game/Blueprints/Interfaces/BPI_PlayerCharacter.RotateTorso`
  (params (Direction :type "Float (double-precision)"))
  (bind _returnvalue (`GameplayStatics.GetWorldDeltaSeconds`))
  (bind _returnvalue_2 (* _returnvalue (`self.TorsoRotationMaxSpeed`)))
  ;[1 0.9979 0.3372] Movement
  (`SceneComponent.K2_AddLocalRotation` (`self.Torso`) (`KismetMathLibrary.MakeRotator` 0.0 0.0 (`KismetMathLibrary.FClamp` (* (* Direction (`self.TorsoRotationSpeed`)) _returnvalue) (* -1.0 _returnvalue_2) _returnvalue_2)) false false))

(event `/Game/Blueprints/Interfaces/BPI_PlayerCharacter.RotateCamera`
  (params (X :type "Float (double-precision)") (Y :type "Float (double-precision)"))
  (bind (_returnvalue_roll _returnvalue_pitch) (`KismetMathLibrary.BreakRotator` (`SceneComponent.K2_GetComponentRotation` (`self.SpringArm`))))
  (bind _returnvalue (`KismetMathLibrary.MakeRotator` 0.0 (* Y -2.5)))
  (bind _returnvalue_2 (+ _returnvalue_pitch (.pitch _returnvalue)))
  ;[1 0.9979 0.3372] Movement
  (if (and (< _returnvalue_2 (`self.CameraMaxRotation`)) (> _returnvalue_2 (`self.CameraMinRotation`)))
    (`SceneComponent.K2_AddLocalRotation` (`self.SpringArm`) _returnvalue false false)))

(event `Key|MouseScrollDown`
  (params (Key :type "Key Structure"))
  ;[1 0 0 1 40] Deprecated
  ;;[1 1 1] Targeting
  ;;;[1 1 1] Manual Targeting Increase distance
)

(event `Key|E`
  (params (Key :type "Key Structure"))
  ;[1 0 0 1 40] Deprecated
  ;;[1 1 1] Targeting
  ;;;[1 1 1] Automatic targeting
)

(event `self.CapsuleComponent.OnComponentBeginOverlap`
  (params (OverlappedComponent :type "PrimitiveComponent Object Reference") (OtherActor :type "Actor Object Reference") (OtherComp :type "PrimitiveComponent Object Reference") (OtherBodyIndex :type Integer) (bFromSweep :type Boolean) (SweepResult :type "HitResult Structure (by ref)"))
  (if (`self.ActorHasTag` OtherActor "DestructibleSmall")
    (message `/Game/Blueprints/Interfaces/BPI_Environment.Damage Building` OtherActor (`SceneComponent.K2_GetComponentLocation` (`Actor.RootComponent` OtherActor)))))

(fn `AimWeapons`
  (params (InputPin :type "Vector Structure"))
  (bind _rightweapon (`self.RightWeapon`))
  (bind _leftweapon (`self.LeftWeapon`))
  (`SceneComponent.K2_SetWorldRotation` _rightweapon (`KismetMathLibrary.FindLookAtRotation` (`SceneComponent.K2_GetComponentLocation` _rightweapon) InputPin) false false)
  (`SceneComponent.K2_SetWorldRotation` _leftweapon (`KismetMathLibrary.FindLookAtRotation` (`SceneComponent.K2_GetComponentLocation` _leftweapon) InputPin) false false)
  (set `self.Location` InputPin))

(fn `GetHeat`
  (returns (CurrentHeat :type "Float (double-precision)") (MaxHeat :type "Float (double-precision)"))
  (return (`self.CurrentHeat`) (`self.MaxHeat`)))

(fn `Handle Hit Enemy`
  (params (OutHit :type "HitResult Structure (by ref)") (IsMinigun :type Boolean))
  (bind (_bblockinghit _binitialoverlap _time _distance _location _impactpoint _normal _impactnormal _physmat _hitactor) (`GameplayStatics.BreakHitResult` OutHit))
  (if (`self.ActorHasTag` _hitactor "EnemyMech")
    (if IsMinigun
      (bind _output_get (set `self.Acan_Damage` 10.0))
      (message `/Game/Blueprints/Interfaces/BPI_EnemyInterface.DamageEnemy` _hitactor _output_get _location)
      (else
        (bind _output_get_2 (set `self.Acan_Damage` 40.0))
        (message `/Game/Blueprints/Interfaces/BPI_EnemyInterface.DamageEnemy` _hitactor _output_get_2 _location))))
  (return))

(fn `Handle Hit Environment`
  (params (`Out Hit` :type "HitResult Structure"))
  (bind (_bblockinghit _binitialoverlap _time _distance _location _impactpoint _normal _impactnormal _physmat _hitactor) (`GameplayStatics.BreakHitResult` `Out Hit`))
  (bind _returnvalue (* (`KismetMathLibrary.Vector_One`) (`KismetMathLibrary.RandomFloatInRange` 3.0 5.0)))
  (if (`KismetSystemLibrary.IsValid` _hitactor)
    (if (`self.ActorHasTag` _hitactor "DestructibleBig")
      (message `/Game/Blueprints/Interfaces/BPI_Environment.Damage Building` _hitactor _location)
      (`GameplayStatics.SpawnEmitterAtLocation` "/Game/Realistic_Starter_VFX_Pack_Vol2/Particles/Destruction/P_Destruction_Concrete.P_Destruction_Concrete" _location (struct) _returnvalue)
      (`GameplayStatics.SpawnEmitterAtLocation` "/Game/Realistic_Starter_VFX_Pack_Vol2/Particles/Destruction/P_Destruction_Building_A.P_Destruction_Building_A" _location (struct) (* _returnvalue 1.5))
      (`GameplayStatics.PlaySoundAtLocation` "/Game/Sounds/Environment/SFX_BuildingImpact1.SFX_BuildingImpact1" _location (struct) 1.0 1.0 0.0 null null null null)
      (return)
      (elif (`self.ActorHasTag` _hitactor "EnvironmentSnow")
        (`GameplayStatics.SpawnEmitterAtLocation` "/Game/Realistic_Starter_VFX_Pack_Vol2/Particles/Hit/P_Ice.P_Ice" _location (`KismetMathLibrary.MakeRotator` 0.0) (5.0 5.0 5.0))
        (return)
        (elif (`self.ActorHasTag` _hitactor "DestructibleSmall")
          (message `/Game/Blueprints/Interfaces/BPI_Environment.Damage Building` _hitactor _location)
          (`GameplayStatics.SpawnEmitterAtLocation` "/Game/Realistic_Starter_VFX_Pack_Vol2/Particles/Destruction/P_Destruction_Concrete.P_Destruction_Concrete" _location (struct) (2.0 2.0 2.0))
          (`GameplayStatics.SpawnEmitterAtLocation` "/Game/Realistic_Starter_VFX_Pack_Vol2/Particles/Destruction/P_Destruction_Building_A.P_Destruction_Building_A" _location (struct) (2.0 2.0 2.0))
          (`GameplayStatics.PlaySoundAtLocation` "/Game/Sounds/Environment/SFX_BuildingImpact1.SFX_BuildingImpact1" _location (struct) 1.0 1.0 0.0 null null null null))))
    (else
      (return))))

(fn `HandleAutoFireLogic`
  (params (weaponTarget :type "SceneComponent Object Reference") (isRightWeapon :type Boolean))
  (bind (_returnvalue_roll _returnvalue_pitch _returnvalue_yaw) (`KismetMathLibrary.BreakRotator` (`SceneComponent.K2_GetComponentRotation` weaponTarget)))
  (bind _returnvalue (`SceneComponent.GetSocketLocation` weaponTarget "Muzzle"))
  (if isRightWeapon
    ;[1 1 1] Right Weapon
    (`NiagaraFunctionLibrary.SpawnSystemAtLocation` "/Game/Graphics/Effects/FX_ShellDrop.FX_ShellDrop" (`SceneComponent.K2_GetComponentLocation` weaponTarget) (`SceneComponent.K2_GetComponentRotation` weaponTarget))
    (`GameplayStatics.SpawnEmitterAtLocation` "/Game/InfinityBladeEffects/Effects/FX_Monsters/FX_Monster_Gruntling/Master/P_BackPack_MuzzleFlash.P_BackPack_MuzzleFlash" (`SceneComponent.GetSocketLocation` (`self.WR_GunBarrel`) "Muzzle"))
    (else
      ;[1 1 1] Left Weapon
      (`NiagaraFunctionLibrary.SpawnSystemAtLocation` "/Game/Graphics/Effects/FX_ShellDrop.FX_ShellDrop" (`SceneComponent.K2_GetComponentLocation` weaponTarget) (`KismetMathLibrary.MakeRotator` _returnvalue_roll _returnvalue_pitch (+ _returnvalue_yaw 180.0)))
      (`GameplayStatics.SpawnEmitterAtLocation` "/Game/InfinityBladeEffects/Effects/FX_Monsters/FX_Monster_Gruntling/Master/P_BackPack_MuzzleFlash.P_BackPack_MuzzleFlash" (`SceneComponent.GetSocketLocation` (`self.WL_GunBarrel`) "Muzzle"))))
  (`GameplayStatics.PlaySoundAtLocation` "/Game/Sounds/Mech/Weapons/Akan40mm/40mmCannonFire1.40mmCannonFire1" (`SceneComponent.K2_GetComponentLocation` weaponTarget) (struct) 1.0 1.0 0.0 null null null null)
  (bind (_outhit _returnvalue_2) (`KismetSystemLibrary.LineTraceSingle` :`Start` _returnvalue :`End` (+ _returnvalue (* (`KismetMathLibrary.GetDirectionUnitVector` _returnvalue (`self.Location`)) (`KismetMathLibrary.Conv_DoubleToVector` 30000.0))) :`TraceChannel` "TraceTypeQuery2" :`DrawDebugType` "ForDuration" :`TraceColor` (struct :`G` 1.0 :`B` 0.246827 :`A` 0.393) :`TraceHitColor` (struct :`R` 0.964683 :`G` 0.046352 :`B` 1.0 :`A` 1.0) :`DrawTime` 3.0))
  (if _returnvalue_2
    (`self.SpawnImpactDecal` _outhit)
    (`self.Handle Hit Enemy` _outhit isRightWeapon)
    (`self.Handle Hit Environment` _outhit)
    (return)))

(fn `SpawnImpactDecal`
  (params (Hit :type "HitResult Structure (by ref)"))
  (bind _returnvalue (`KismetMathLibrary.RandomIntegerInRange` 0 2))
  (bind _returnvalue_2 (`KismetMathLibrary.RandomFloatInRange` 40.0 100.0))
  (bind (_bblockinghit _binitialoverlap _time _distance _location _impactpoint _normal _impactnormal _physmat _hitactor _hitcomponent) (`GameplayStatics.BreakHitResult` Hit))
  (if (== _returnvalue 0)
    (set `self.Decal Material` "/Game/Graphics/Materials/BulletHoles/M_bulletImpactHole1.M_bulletImpactHole1")
    (elif (== _returnvalue 1)
      (set `self.Decal Material` "/Game/Graphics/Materials/BulletHoles/M_bulletImpactHole2.M_bulletImpactHole2")
      (else
        (set `self.Decal Material` "/Game/Graphics/Materials/BulletHoles/M_bulletImpactHole1.M_bulletImpactHole1"))))
  (`GameplayStatics.SpawnDecalAttached` (`self.Decal Material`) (`KismetMathLibrary.MakeVector` _returnvalue_2 _returnvalue_2 _returnvalue_2) _hitcomponent "None" _impactpoint (`KismetMathLibrary.Conv_VectorToRotator` _impactnormal) "KeepWorldPosition" 20.0))

(fn `UserConstructionScript`)