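; Game mode for the Swarm game that owns the HUD and menu flow for pausing and player death.
; BeginPlay creates the pause, game-over and crosshair widgets, adds them to the viewport and keeps the two menus hidden.
; PauseGame and UnPauseGame toggle the pause menu, crosshair, mouse cursor and game pause together.
; PlayerDied only reveals the game-over menu, without pausing or showing the cursor.
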(event `self.ReceiveBeginPlay`
  ;[1 1 1] Init
  (`KismetSystemLibrary.PrintString` "GameMode is GM_Swarm")
  (bind _returnvalue (`|GenericCreateObject` "/Game/Blueprints/Widgets/WBP_PauseMenu.WBP_PauseMenu_C"))
  (bind _returnvalue_2 (`|GenericCreateObject` "/Game/Blueprints/Widgets/WBP_GameOverMenu.WBP_GameOverMenu_C"))
  (`UserWidget.AddToViewport` _returnvalue 0)
  (`UserWidget.AddToViewport` _returnvalue_2 0)
  (bind _output_get (set `self.Pause Menu Ref` _returnvalue))
  (bind _output_get_2 (set `self.Game Over Menu Ref` _returnvalue_2))
  (`Widget.SetVisibility` _output_get "Hidden")
  (`Widget.SetVisibility` _output_get_2 "Hidden")
  (bind _returnvalue_3 (`|CreateWidget` "/Game/Blueprints/Widgets/WBP_Crosshair.WBP_Crosshair_C"))
  (bind _output_get_3 (set `self.Crosshair_Ref` _returnvalue_3))
  (`UserWidget.AddToViewport` _output_get_3 0))

(event `PauseGame`
  ;[1 1 1] Pause
  (set `PlayerController.bShowMouseCursor` true (`GameplayStatics.GetPlayerController` 0))
  (`Widget.SetVisibility` (`self.Pause Menu Ref`) "Visible")
  (`Widget.SetVisibility` (`self.Crosshair_Ref`) "Hidden")
  (`GameplayStatics.SetGamePaused` true))

(event `UnPauseGame`
  ;[1 1 1] Pause
  (set `PlayerController.bShowMouseCursor` false (`GameplayStatics.GetPlayerController` 0))
  (`Widget.SetVisibility` (`self.Pause Menu Ref`) "Hidden")
  (`Widget.SetVisibility` (`self.Crosshair_Ref`) "Visible")
  (`GameplayStatics.SetGamePaused` false))

(event `/Game/Blueprints/Interfaces/BPI_GameModeInterface.PlayerDied`
  (params (PlayerNumber :type Integer))
  (`Widget.SetVisibility` (`self.Game Over Menu Ref`) "Visible"))

(fn `UserConstructionScript`)