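; Player mech character Blueprint whose legs and torso turn independently.
; MoveLegs adds movement input along the Legs' forward X/Y, scaled by direction and leg speed.
; RotateLegs and RotateTorso add their input to the world yaw of their component, keeping pitch and roll, with the torso using mouse X.
; Unconnected controller-input and torso-rotation nodes, including speed/drag scaling, never run.
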(event `MoveLegs`
  (params (Direction :type "Float (double-precision)"))
  (bind (_returnvalue_x _returnvalue_y) (`KismetMathLibrary.BreakVector` (`SceneComponent.GetForwardVector` (`self.Legs`))))
  (`self.AddMovementInput` (`KismetMathLibrary.MakeVector` _returnvalue_x _returnvalue_y) (* Direction (`self.LegMoveSpeed`))))

(event `RotateLegs`
  (params (Direction :type "Float (double-precision)"))
  (`SceneComponent.K2_SetWorldRotation` (`self.Legs`) (`KismetMathLibrary.MakeRotator` (.roll (`SceneComponent.K2_GetComponentRotation` (`self.Legs`))) (.pitch (`SceneComponent.K2_GetComponentRotation` (`self.Legs`))) (+ (.yaw (`SceneComponent.K2_GetComponentRotation` (`self.Legs`))) Direction)) false false))

(event `RotateTorso`
  (params (MouseDirections :type "Vector2D Structure"))
  (`SceneComponent.K2_SetWorldRotation` (`self.Torso`) (`KismetMathLibrary.MakeRotator` (.roll (`SceneComponent.K2_GetComponentRotation` (`self.Torso`))) (.pitch (`SceneComponent.K2_GetComponentRotation` (`self.Torso`))) (+ (.yaw (`SceneComponent.K2_GetComponentRotation` (`self.Torso`))) MouseDirections_X)) false false))

(fn `UserConstructionScript`)