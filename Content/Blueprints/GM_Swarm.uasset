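; GM_Swarm is the game mode for a wave-based enemy mode, handling wave progression, pause and win/lose screens.
; On start it creates the menu and crosshair widgets, finds the BP_EnemySpawner and requests the first wave from the Waves array.
; Further waves are requested after a post-spawn delay or when all tracked enemies die, gated by a NAND of waves-remaining and IsSpawning.
; Clearing enemies with no waves left triggers victory.
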(event `self.ReceiveBeginPlay`
  ;[1 1 1] Init
  (`KismetSystemLibrary.PrintString` "GameMode is GM_Swarm")
  (bind _returnvalue (`|GenericCreateObject` "/Game/Blueprints/Widgets/WBP_PauseMenu.WBP_PauseMenu_C"))
  (bind _returnvalue_2 (`|GenericCreateObject` "/Game/Blueprints/Widgets/WBP_GameOverMenu.WBP_GameOverMenu_C"))
  (`UserWidget.AddToViewport` _returnvalue 0)
  (`UserWidget.AddToViewport` _returnvalue_2 0)
  (bind _output_get (set `self.Pause Menu Ref` _returnvalue))
  (bind _output_get_2 (set `self.Game Over Menu Ref` _returnvalue_2))
  (`Widget.SetVisibility` _output_get "Hidden")
  (`Widget.SetVisibility` _output_get_2 "Hidden")
  (bind _returnvalue_3 (`|CreateWidget` "/Game/Blueprints/Widgets/WBP_Crosshair.WBP_Crosshair_C"))
  (bind _output_get_3 (set `self.Crosshair_Ref` _returnvalue_3))
  (`UserWidget.AddToViewport` _output_get_3 0)
  (bind _returnvalue_4 (`GameplayStatics.GetActorOfClass` "/Game/Blueprints/Enemy/BP_EnemySpawner.BP_EnemySpawner_C"))
  (set `self.EnemySpawner` _returnvalue_4)
  (`self.QueryShouldSpawnNewWave`))

(event `PauseGame`
  ;[1 1 1] Pause
  (set `PlayerController.bShowMouseCursor` true (`GameplayStatics.GetPlayerController` 0))
  (`Widget.SetVisibility` (`self.Pause Menu Ref`) "Visible")
  (`Widget.SetVisibility` (`self.Crosshair_Ref`) "Hidden")
  (`GameplayStatics.SetGamePaused` true))

(event `UnPauseGame`
  ;[1 1 1] Pause
  (set `PlayerController.bShowMouseCursor` false (`GameplayStatics.GetPlayerController` 0))
  (`Widget.SetVisibility` (`self.Pause Menu Ref`) "Hidden")
  (`Widget.SetVisibility` (`self.Crosshair_Ref`) "Visible")
  (`GameplayStatics.SetGamePaused` false))

(event `/Game/Blueprints/Interfaces/BPI_GameModeInterface.EnemySpawned`
  (params (EnemyCharacter_Ref :type "Character Object Reference"))
  ;[1 0.1615 0.1615] Enemy Logic
  ;;[0.3265 1 0.5582] Spawn Logic
  ;;;[1 1 1 0.717] Spawned
  (`KismetArrayLibrary.Array_AddUnique` (`self.Enemies`) EnemyCharacter_Ref))

(event `SpawnWave`
  ;[1 0.1615 0.1615] Enemy Logic
  ;;[0.3265 1 0.5582] Spawn Logic
  ;;;[1 1 1] Spawn next wave
  (`/Game/Blueprints/Enemy/BP_EnemySpawner.SpawnEnemies` (`self.EnemySpawner`) (`|GetArrayItem` (`self.Waves`) (`self.WaveCount`))))

(event `/Game/Blueprints/Interfaces/BPI_GameModeInterface.EnemiesFinishedSpawning`
  (bind _timebeforenextwavespawn (`self.TimeBeforeNextWaveSpawn`))
  ;[1 0.1615 0.1615] Enemy Logic
  ;;[0.3265 1 0.5582] Spawn Logic
  ;;;[1 1 1] Finished Spawning
  (`/Engine/EditorBlueprintResources/StandardMacros.IncrementInt` (`self.WaveCount`)
    (:`  `
      (`KismetSystemLibrary.PrintString` (`KismetStringLibrary.Concat_StrStr` "Next Spawn in: {" (`KismetStringLibrary.Conv_DoubleToString` _timebeforenextwavespawn) "} seconds!") true true (struct :`R` 0.98344 :`G` 1.0 :`A` 1.0) 5.0)
      (`KismetSystemLibrary.Delay` _timebeforenextwavespawn)
      (if (not (`/Game/Blueprints/Enemy/BP_EnemySpawner.IsSpawning` (`self.EnemySpawner`)))
        (`self.QueryShouldSpawnNewWave`)))))

(event `QueryShouldSpawnNewWave`
  ;[1 0.1615 0.1615] Enemy Logic
  ;;[0.3265 1 0.5582] Spawn Logic
  ;;;[1 1 1 0.717] Wave Condition
  (bind _result (`self.CanStillSpawnWaves`))
  (if (`KismetMathLibrary.BooleanNAND` _result (`/Game/Blueprints/Enemy/BP_EnemySpawner.IsSpawning` (`self.EnemySpawner`)))
    (`self.SpawnWave`)))

(event `/Game/Blueprints/Interfaces/BPI_GameModeInterface.EnemyKilled`
  (params (EnemyCharacter_Ref :type "Character Object Reference"))
  (bind _enemies (`self.Enemies`))
  ;[1 0.1615 0.1615] Enemy Logic
  ;;[1 1 1 0.717] Killed
  (if (`/Game/Blueprints/Global/ExtraMacros.DoesItemExist` EnemyCharacter_Ref (`self.Enemies`))
    (`KismetArrayLibrary.Array_RemoveItem` _enemies EnemyCharacter_Ref)
    (if (<= (`KismetArrayLibrary.Array_Length` _enemies) 0)
      (bind _result (`self.CanStillSpawnWaves`))
      (if _result
        (`self.QueryShouldSpawnNewWave`)
        (else
          (`self.TriggerWinState`))))))

(event `/Game/Blueprints/Interfaces/BPI_GameModeInterface.PlayerDied`
  (params (PlayerNumber :type Integer))
  (bind _game_over_menu_ref (`self.Game Over Menu Ref`))
  (`/Game/Blueprints/Widgets/WBP_GameOverMenu.PlayerLose` _game_over_menu_ref)
  (`Widget.SetVisibility` _game_over_menu_ref "Visible")
  (set `PlayerController.bShowMouseCursor` true (`GameplayStatics.GetPlayerController` 0)))

(event `TriggerWinState`
  (bind _game_over_menu_ref (`self.Game Over Menu Ref`))
  (`/Game/Blueprints/Widgets/WBP_GameOverMenu.PlayerWin` _game_over_menu_ref)
  (`Widget.SetVisibility` _game_over_menu_ref "Visible")
  (set `PlayerController.bShowMouseCursor` true (`GameplayStatics.GetPlayerController` 0)))

(fn `CanStillSpawnWaves`
  (returns (Result :type Boolean))
  (return (< (`self.WaveCount`) (`KismetArrayLibrary.Array_Length` (`self.Waves`)))))

(fn `UserConstructionScript`)