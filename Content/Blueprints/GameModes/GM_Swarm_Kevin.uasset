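; Game mode for the Swarm wave mode that handles UI, pausing, score and win/lose states.
; After a one-second BeginPlay delay, it caches BP_EnemyWaveSpawner and creates pause, game-over and crosshair widgets.
; Events toggle pause or show the end screen, while EnemyKilled adds score and notifies the spawner, which also supplies round and living-enemy getters.
; The older in-mode wave logic is deprecated, with empty events and disconnected nodes.
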(event `self.ReceiveBeginPlay`
  ;[1 1 1] Init
  (`KismetSystemLibrary.Delay` 1.0) ; Needed for when reloading a level for some reason
  (`KismetSystemLibrary.PrintString` "GameMode is GM_Swarm")
  (bind _returnvalue (`GameplayStatics.GetActorOfClass` "/Game/Blueprints/Enemy/BP_EnemyWaveSpawner.BP_EnemyWaveSpawner_C"))
  (set `self.enemyWaveSpawner` _returnvalue)
  ;[1 1 1] Viewport
  (bind _returnvalue_2 (`|GenericCreateObject` "/Game/Blueprints/Widgets/WBP_PauseMenu.WBP_PauseMenu_C"))
  (bind _returnvalue_3 (`|GenericCreateObject` "/Game/Blueprints/Widgets/WBP_GameOverMenu.WBP_GameOverMenu_C"))
  (`UserWidget.AddToViewport` _returnvalue_2 0)
  (`UserWidget.AddToViewport` _returnvalue_3 0)
  (bind _output_get (set `self.Pause Menu Ref` _returnvalue_2))
  (bind _output_get_2 (set `self.Game Over Menu Ref` _returnvalue_3))
  (`Widget.SetVisibility` _output_get "Hidden")
  (`Widget.SetVisibility` _output_get_2 "Hidden")
  (bind _returnvalue_4 (`|CreateWidget` "/Game/Blueprints/Widgets/WBP_Crosshair.WBP_Crosshair_C"))
  (bind _output_get_3 (set `self.Crosshair_Ref` _returnvalue_4))
  (`UserWidget.AddToViewport` _output_get_3 0))

(event `PauseGame`
  ;[1 1 1] Pause
  (set `PlayerController.bShowMouseCursor` true (`GameplayStatics.GetPlayerController` 0))
  (`Widget.SetVisibility` (`self.Pause Menu Ref`) "Visible")
  (`Widget.SetVisibility` (`self.Crosshair_Ref`) "Hidden")
  (`GameplayStatics.SetGamePaused` true))

(event `UnPauseGame`
  ;[1 1 1] Pause
  (set `PlayerController.bShowMouseCursor` false (`GameplayStatics.GetPlayerController` 0))
  (`Widget.SetVisibility` (`self.Pause Menu Ref`) "Hidden")
  (`Widget.SetVisibility` (`self.Crosshair_Ref`) "Visible")
  (`GameplayStatics.SetGamePaused` false))

(event `/Game/Blueprints/Interfaces/BPI_GameModeInterface.PlayerDied`
  (params (PlayerNumber :type Integer))
  (bind _game_over_menu_ref (`self.Game Over Menu Ref`))
  ;[1 1 1] WinLose State
  (`/Game/Blueprints/Widgets/WBP_GameOverMenu.PlayerLose` _game_over_menu_ref)
  (`Widget.SetVisibility` _game_over_menu_ref "Visible")
  (set `PlayerController.bShowMouseCursor` true (`GameplayStatics.GetPlayerController` 0))
  (`GameplayStatics.SetGamePaused` true :!label _label))

(event `TriggerWinState`
  (bind _game_over_menu_ref (`self.Game Over Menu Ref`))
  ;[1 1 1] WinLose State
  (`/Game/Blueprints/Widgets/WBP_GameOverMenu.PlayerWin` _game_over_menu_ref)
  (`Widget.SetVisibility` _game_over_menu_ref "Visible")
  (set `PlayerController.bShowMouseCursor` true (`GameplayStatics.GetPlayerController` 0))
  (goto _label))

(event `/Game/Blueprints/Interfaces/BPI_GameModeInterface.EnemyKilled`
  (params (EnemyCharacter_Ref :type "Character Object Reference"))
  (set `self.PlayerScore` (+ (`self.PlayerScore`) 10))
  (`/Game/Blueprints/Enemy/BP_EnemyWaveSpawner.EnemyKilled` (`self.enemyWaveSpawner`)))

(event `/Game/Blueprints/Interfaces/BPI_GameModeInterface.EnemySpawned`
  (params (EnemyCharacter_Ref :type "Character Object Reference"))
  ;[1 0 0 1 80] DEPRECATED
  ;;[1 0.1615 0.1615] Enemy Logic
  ;;;[0.3265 1 0.5582] Spawn Logic
  ;;;;[1 1 1 0.717] Spawned
)

(event `SpawnWave`
  ;[1 0 0 1 80] DEPRECATED
  ;;[1 0.1615 0.1615] Enemy Logic
  ;;;[0.3265 1 0.5582] Spawn Logic
  ;;;;[1 1 1] Spawn next wave
)

(event `/Game/Blueprints/Interfaces/BPI_GameModeInterface.EnemiesFinishedSpawning`
  ;[1 0 0 1 80] DEPRECATED
  ;;[1 0.1615 0.1615] Enemy Logic
  ;;;[0.3265 1 0.5582] Spawn Logic
  ;;;;[1 1 1] Finished Spawning
)

(event `QueryShouldSpawnNewWave`
  ;[1 0 0 1 80] DEPRECATED
  ;;[1 0.1615 0.1615] Enemy Logic
  ;;;[0.3265 1 0.5582] Spawn Logic
  ;;;;[1 1 1 0.717] Wave Condition
)

(fn `CanStillSpawnWaves`
  (returns (Result :type Boolean))
  (return (< (`self.WaveCount`) (`KismetArrayLibrary.Array_Length` (`self.Waves`)))))

(fn `GetCurrentRound`
  (returns (CurrentRound :type Integer))
  (return (`/Game/Blueprints/Enemy/BP_EnemyWaveSpawner.currentRound` (`self.enemyWaveSpawner`))))

(fn `GetEnemiesCount`
  (returns (Count :type Integer))
  (return (`/Game/Blueprints/Enemy/BP_EnemyWaveSpawner.currentLivingEnemies` (`self.enemyWaveSpawner`))))

(fn `GetPlayerScore`
  (returns (Score :type Integer))
  (return (`self.PlayerScore`)))

(fn `UserConstructionScript`)