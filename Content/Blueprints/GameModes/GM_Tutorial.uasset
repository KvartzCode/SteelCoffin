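; Tutorial game mode that tracks stationary targets and AI enemies, and shows the game-over message on the HUD when the player dies.
; After a delayed init, it counts BP_EnemyCube targets; SpawnEnemies places tutorial mechs at tagged TargetPoints and counts them.
; EnemyKilled decrements the matching counter and signals when either group is cleared.
; Getters expose score, plus round and living-enemy count from a cached wave spawner, defaulting to zero without one.
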(event `self.ReceiveBeginPlay`
  ;[1 1 1] Init
  (`KismetSystemLibrary.Delay` 1.0) ; Needed for when reloading a level for some reason
  (`KismetSystemLibrary.PrintString` "GameMode is GM_Swarm")
  (bind _returnvalue (`GameplayStatics.GetActorOfClass` "/Game/Blueprints/Enemy/BP_EnemyWaveSpawner.BP_EnemyWaveSpawner_C"))
  (set `self.EnemyWaveSpawner` _returnvalue)
  (bind _outactors (`GameplayStatics.GetAllActorsOfClass` "/Game/Blueprints/Enemy/TutorialEnemy/BP_EnemyCube.BP_EnemyCube_C"))
  (set `self.StationaryTargetCount` (`KismetArrayLibrary.Array_Length` _outactors)))

(event `/Game/Blueprints/Interfaces/BPI_GameModeInterface.PlayerDied`
  (params (PlayerNumber :type Integer))
  ;[1 1 1] Player Death
  (message `/Game/Blueprints/Interfaces/BPI_HUDMaster.ShowGameOverScreen` (`PlayerController.GetHUD` (`GameplayStatics.GetPlayerController` 0))))

(event `/Game/Blueprints/Interfaces/BPI_GameModeInterface.EnemyKilled`
  (params (IsTurret :type Boolean))
  ;[1 1 1] Enemy Killed
  (if IsTurret
    (bind _result (`/Engine/EditorBlueprintResources/StandardMacros.DecrementInt` (`self.StationaryTargetCount`))
      (:`  `
        (if (<= _result 0)
          (`self.StationaryTargetsDestroyed`))))
    (else
      (bind _result_2 (`/Engine/EditorBlueprintResources/StandardMacros.DecrementInt` (`self.AIEnemyCount`))
        (:`  `
          (if (<= _result_2 0)
            (`self.AIEnemiesDestroyed`)))))))

(event `SpawnEnemies`
  ;[1 1 1] Spawn Enemies
  (bind _outactors (`GameplayStatics.GetAllActorsOfClassWithTag` "/Script/Engine.TargetPoint" "SpawnPoint"))
  (for _array_element _outactors
    (`|SpawnActorFromClass` "/Game/Blueprints/Enemy/TutorialEnemy/BP_EnemyMechTutorial.BP_EnemyMechTutorial_C" (`self.GetTransform` _array_element) "AdjustIfPossibleButAlwaysSpawn" "OverrideRootScale" null null)
    (`/Engine/EditorBlueprintResources/StandardMacros.IncrementInt` (`self.AIEnemyCount`))))

(fn `GetCurrentRound`
  (returns (CurrentRound :type Integer))
  (bind _enemywavespawner (`self.EnemyWaveSpawner`))
  (if (`KismetSystemLibrary.IsValid` _enemywavespawner)
    (return (`/Game/Blueprints/Enemy/BP_EnemyWaveSpawner.currentRound` _enemywavespawner))
    (else
      (return 0))))

(fn `GetEnemiesCount`
  (returns (Count :type Integer))
  (bind _enemywavespawner (`self.EnemyWaveSpawner`))
  (if (`KismetSystemLibrary.IsValid` _enemywavespawner)
    (return (`/Game/Blueprints/Enemy/BP_EnemyWaveSpawner.currentLivingEnemies` _enemywavespawner))
    (else
      (return 0))))

(fn `GetPlayerScore`
  (returns (Score :type Integer))
  (return (`self.PlayerScore`)))

(fn `UserConstructionScript`)