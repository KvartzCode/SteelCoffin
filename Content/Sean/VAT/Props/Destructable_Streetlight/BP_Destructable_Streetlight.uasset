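; Destructible streetlight prop that drives vertex animation texture (VAT) destruction from a hit location.
; DamageBuilding passes the local-space hit position and time to materials drawing into two small float render targets, this and previous frame, feeding the mesh's VAT material.
; Tick keeps redrawing both targets while updating is active.
; The first hit destroys the spotlight, then after a short delay zeroes emission, stops updates and disables collision.
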(event `self.ReceiveBeginPlay`
  (bind _staticmesh (`self.StaticMesh`))
  (bind _returnvalue (`PrimitiveComponent.CreateDynamicMaterialInstance` _staticmesh 0 (`PrimitiveComponent.GetMaterial` _staticmesh 0) "None"))
  (set `self.VAT MID` _returnvalue)
  (bind _returnvalue_2 (`KismetMaterialLibrary.CreateDynamicMaterialInstance` (`self.RT Drawing Prev MI`)))
  (set `self.RT Drawing Prev MID` _returnvalue_2)
  (bind _returnvalue_3 (`KismetMaterialLibrary.CreateDynamicMaterialInstance` (`self.RT Drawing This MI`)))
  (set `self.RT Drawing This MID` _returnvalue_3)
  (bind _returnvalue_4 (`KismetRenderingLibrary.CreateRenderTarget2D` 128 3 "RTF_RGBA32f"))
  (set `self.RT Prev Frame` _returnvalue_4)
  (bind _returnvalue_5 (`KismetRenderingLibrary.CreateRenderTarget2D` 128 3 "RTF_RGBA32f"))
  (bind _output_get (set `self.RT This Frame` _returnvalue_5))
  (`MaterialInstanceDynamic.SetTextureParameterValue` (`self.RT Drawing Prev MID`) "RT This Frame" _output_get)
  (`MaterialInstanceDynamic.SetTextureParameterValue` (`self.RT Drawing This MID`) "RT Prev Frame" (`self.RT Prev Frame`))
  (`MaterialInstanceDynamic.SetTextureParameterValue` (`self.VAT MID`) "RT" (`self.RT This Frame`))
  (bind _returnvalue_6 (`PrimitiveComponent.CreateDynamicMaterialInstance` (`self.StaticMesh`) 0 null "None")))

(event `/Game/Blueprints/Interfaces/BPI_Environment.Damage Building`
  (params (HitLocation :type "Vector Structure"))
  (bind _rt_drawing_this_mid (`self.RT Drawing This MID`))
  (set `self.ShouldUpdateRT` true)
  (set `self.ProjectileLocation` HitLocation)
  (`MaterialInstanceDynamic.SetVectorParameterValue` _rt_drawing_this_mid "Overlap Local Position" (make `LinearColor` (.x (`KismetMathLibrary.InverseTransformLocation` (`SceneComponent.K2_GetComponentToWorld` (`self.DefaultSceneRoot`)) (`self.ProjectileLocation`))) (.y (`KismetMathLibrary.InverseTransformLocation` (`SceneComponent.K2_GetComponentToWorld` (`self.DefaultSceneRoot`)) (`self.ProjectileLocation`))) (.z (`KismetMathLibrary.InverseTransformLocation` (`SceneComponent.K2_GetComponentToWorld` (`self.DefaultSceneRoot`)) (`self.ProjectileLocation`))) 1.0))
  (`MaterialInstanceDynamic.SetScalarParameterValue` _rt_drawing_this_mid "Game Time" (`GameplayStatics.GetTimeSeconds`))
  (`KismetRenderingLibrary.DrawMaterialToRenderTarget` (`self.RT This Frame`) (`self.RT Drawing This MID`))
  (`KismetRenderingLibrary.DrawMaterialToRenderTarget` (`self.RT Prev Frame`) (`self.RT Drawing Prev MID`))
  (`|ExecutionSequence`
    (:`then_0`
      (`/Engine/EditorBlueprintResources/StandardMacros.DoOnce` false
        (:`Completed`
          (`KismetSystemLibrary.SphereTraceSingle` (0.0 0.0 0.0) (0.0 0.0 0.0) 0.0 "TraceTypeQuery1")
          (`ActorComponent.K2_DestroyComponent` (`self.SpotLight`))
          (`KismetSystemLibrary.Delay` 0.3)
          (`MaterialInstanceDynamic.SetScalarParameterValue` (stale `self.ReceiveBeginPlay` _returnvalue_6) "EmissionStrength" 0.0)
          (set `self.ShouldUpdateRT` false)
          (`self.SetActorEnableCollision` false))))
    (:`then_1`
      (`KismetSystemLibrary.PrintString` "Hit!"))))

(event `self.ReceiveActorEndOverlap`
  (params (OtherActor :type "Actor Object Reference")))

(event `self.ReceiveHit`
  (params (MyComp :type "PrimitiveComponent Object Reference") (Other :type "Actor Object Reference") (OtherComp :type "PrimitiveComponent Object Reference") (bSelfMoved :type Boolean) (HitLocation :type "Vector Structure") (HitNormal :type "Vector Structure") (NormalImpulse :type "Vector Structure") (Hit :type "HitResult Structure (by ref)")))

(event `self.ReceiveTick`
  (params (DeltaSeconds :type "Float (single-precision)"))
  (bind _rt_drawing_this_mid (`self.RT Drawing This MID`))
  (if (`self.ShouldUpdateRT`)
    (`MaterialInstanceDynamic.SetVectorParameterValue` _rt_drawing_this_mid "Overlap Local Position" (make `LinearColor` (.x (`KismetMathLibrary.InverseTransformLocation` (`SceneComponent.K2_GetComponentToWorld` (`self.DefaultSceneRoot`)) (`self.ProjectileLocation`))) (.y (`KismetMathLibrary.InverseTransformLocation` (`SceneComponent.K2_GetComponentToWorld` (`self.DefaultSceneRoot`)) (`self.ProjectileLocation`))) (.z (`KismetMathLibrary.InverseTransformLocation` (`SceneComponent.K2_GetComponentToWorld` (`self.DefaultSceneRoot`)) (`self.ProjectileLocation`))) 1.0))
    (`MaterialInstanceDynamic.SetScalarParameterValue` _rt_drawing_this_mid "Game Time" (`GameplayStatics.GetTimeSeconds`))
    (`KismetRenderingLibrary.DrawMaterialToRenderTarget` (`self.RT This Frame`) (`self.RT Drawing This MID`))
    (`KismetRenderingLibrary.DrawMaterialToRenderTarget` (`self.RT Prev Frame`) (`self.RT Drawing Prev MID`))))

(fn `UserConstructionScript`)